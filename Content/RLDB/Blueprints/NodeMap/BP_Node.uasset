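; BP_Node is a clickable encounter node on the node map, showing an icon by GameplayTag and spline-mesh edges to its connected nodes, built in the construction script.
; Enabled nodes wobble via a gated looping timeline and highlight on hover through a dynamic material.
; Clicking records the visit, then either fades out and loads a random arena from the tier's DataTable, heals persistent heroes, or plays a treasure card, saving after the latter two.
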(event `self.ReceiveBeginPlay`
  ;[0 0 0] Store original node color on startup
  (bind _returnvalue (`MaterialInstanceDynamic.K2_GetVectorParameterValue` (`self.NodeMaterial`) "Color"))
  (set `self.TrueColor` _returnvalue))

(event `CrossOut`
  ;[0 0 0] Visualizing node having been visited by crossing it out
  (`SceneComponent.SetVisibility` (`self.CrossMesh`) true false))

(event `Enable`
  ;[0 0 0] Signals that node can be clicked and starts wobble animation to communicate this to the player
  (set `self.bEnabled` true)
  (`|ExecutionSequence`
    (:`then_0`
      (goto _label_2 :!via `Open`))
    (:`then_1`
      (bind (_direction _wobble) (`Timeline|TL_Wobble` :!via `PlayFromStart` :!label _label)
        (:`Update`
          (`SceneComponent.SetRelativeScale3D` (`self.NodeMesh`) (`KismetMathLibrary.Conv_DoubleToVector` (+ 1.0 (* _wobble 0.2)))))
        (:`Finished`
          (`/Engine/EditorBlueprintResources/StandardMacros.Gate` true :!label _label_2
            (:`Exit`
              (goto _label :!via `PlayFromStart`))))))))

(event `StopEnable`
  ;[0 0 0] Signals that node can be clicked and starts wobble animation to communicate this to the player
  (set `self.bEnabled` false)
  (goto _label_2 :!via `Close`))

(event `/Game/RLDB/Blueprints/Interfaces/BPI_Node.HoverOverNode`
  ;[0 0 0] Handles mouse over highlighting
  (if (`self.bEnabled`)
    (bind _returnvalue (`MaterialInstanceDynamic.K2_GetVectorParameterValue` (`self.NodeMaterial`) "Color"))
    (set `self.TrueColor` _returnvalue)
    (`MaterialInstanceDynamic.SetVectorParameterValue` (`self.NodeMaterial`) "Color" (struct :`R` 1.0 :`G` 1.0 :`B` 1.0 :`A` 1.0))))

(event `/Game/RLDB/Blueprints/Interfaces/BPI_Node.HoverOffNode`
  ;[0 0 0] Handles mouse over highlighting
  (if (`self.bEnabled`)
    (`MaterialInstanceDynamic.SetVectorParameterValue` (`self.NodeMaterial`) "Color" (`self.TrueColor`))))

(event `/Game/RLDB/Blueprints/Interfaces/BPI_Node.ClickNode`
  ;[0 0 0] Resolve result of clicking node, based on the node GameplayTag, including loading arena maps
  (if (`self.bEnabled`)
    (message `/Game/RLDB/Blueprints/Interfaces/BPI_CardGameInstance.AddVisitedNodeToInstance` (`GameplayStatics.GetGameInstance`) (`self.Id`))
    (`self.OnNodeSelected` self)
    (`|SwitchGameplayTag` (`self.GameplayTag`)
      (:`Default`
        (bind _returnvalue (`|CreateWidget` "/Game/RLDB/Widgets/WBP_ScreenFade.WBP_ScreenFade_C" :!label _label_3))
        (`UserWidget.AddToViewport` _returnvalue 0)
        (bind _occlude (`/Game/RLDB/Widgets/WBP_ScreenFade.Occlude` _returnvalue))
        (`UserWidget.PlayAnimation` _returnvalue _occlude 0.0 1 "Forward" 1.0 false)
        (`KismetSystemLibrary.Delay` (+ (`WidgetAnimation.GetEndTime` _occlude) 0.01))
        (`self.SetupAndLoadArena`))
      (:`Encounter.Easy`
        (goto _label_3))
      (:`Encounter.Normal`
        (goto _label_3))
      (:`Encounter.Elite`
        (goto _label_3))
      (:`Encounter.Boss`
        (goto _label_3))
      (:`Encounter.Rest`
        (`self.HealHeroes` (`self.Heal Amount`))
        (bind _returnvalue_2 (`GameplayStatics.GetCurrentLevelName` true))
        (message `/Game/RLDB/Blueprints/Interfaces/BPI_CardGameInstance.AttemptSaveGame` (`GameplayStatics.GetGameInstance`) _returnvalue_2))
      (:`Encounter.Treasure`
        (bind _returnvalue_3 (`|SpawnActorFromClass` "/Game/RLDB/Blueprints/Core/BP_Card.BP_Card_C" (`KismetMathLibrary.MakeTransform` (0.0 0.0 0.0)) "AlwaysSpawn" "OverrideRootScale" null (`/Game/RLDB/Blueprints/Libraries/BPFL_Card.MakeCardStructFromCardData` (make `DataTableRowHandle` "/Game/RLDB/Data/Cards/DT_Cards_Unobtainable.DT_Cards_Unobtainable" "Treasure")) null))
        (`/Game/RLDB/Blueprints/Core/BP_Card.AttemptUseCard` _returnvalue_3 (`|MakeArray` null :!type "Actor Object Reference") false false)
        (bind _returnvalue_4 (`GameplayStatics.GetCurrentLevelName` true))
        (message `/Game/RLDB/Blueprints/Interfaces/BPI_CardGameInstance.AttemptSaveGame` (`GameplayStatics.GetGameInstance`) _returnvalue_4)))))

(fn `AddConnectionSplines`
  (bind _returnvalue (`self.K2_GetActorLocation`))
  (for _array_element (`self.Connections`)
    (`/Engine/EditorBlueprintResources/StandardMacros.IsValid` _array_element
      (:`Is Valid`
        (bind _returnvalue_2 (`AddComponent|NODE_AddSplineComponent-1`))
        (bind _returnvalue_3 (`self.K2_GetActorLocation` _array_element))
        (bind _returnvalue_4 (* (`KismetMathLibrary.Normal` (- _returnvalue_3 _returnvalue)) 50.0))
        (`SplineComponent.SetLocationAtSplinePoint` _returnvalue_2 0 (+ _returnvalue _returnvalue_4) "World" true)
        (`SplineComponent.SetLocationAtSplinePoint` _returnvalue_2 (- (`SplineComponent.GetNumberOfSplinePoints` _returnvalue_2) 1) (- _returnvalue_3 _returnvalue_4) "World" true)
        (`self.DisplaySplinePath` _returnvalue_2))))
  (return))

(fn `DisplaySplinePath`
  (params (Spline :type "SplineComponent Object Reference"))
  (locals (Divisor :type "Float (double-precision)" :default 64.0))
  (bind _spline (`local.Spline`))
  (for _index (range (+ (`.ReturnValue` (`KismetMathLibrary.FMod` (`SplineComponent.GetSplineLength` Spline) (`local.Divisor`))) 1))
    (bind _returnvalue (`AddComponent|NODE_AddSplineMeshComponent-1` :`bManualAttachment` true))
    (`StaticMeshComponent.SetStaticMesh` _returnvalue "/Game/RLDB/Demo/Meshes/SM_Edge.SM_Edge")
    (bind _returnvalue_2 (* _index (`local.Divisor`)))
    (bind _returnvalue_3 (+ _returnvalue_2 (`local.Divisor`)))
    (`SplineMeshComponent.SetStartAndEnd` _returnvalue (`SplineComponent.GetLocationAtDistanceAlongSpline` _spline _returnvalue_2 "World") (`SplineComponent.GetDirectionAtDistanceAlongSpline` _spline _returnvalue_2 "World") (`SplineComponent.GetLocationAtDistanceAlongSpline` _spline _returnvalue_3 "World") (`SplineComponent.GetDirectionAtDistanceAlongSpline` _spline _returnvalue_3 "World") true))
  (return))

(fn `HealHeroes`
  (params (HealAmount :type Integer))
  (locals (LocalStatuses :type "Map of /Game/RLDB/Blueprints/Statuses/BP_Status Class Reference to Integer"))
  (bind _persistentheroes (message `/Game/RLDB/Blueprints/Interfaces/BPI_CardGameInstance.GetPersistentHeroesFromInstance` (`GameplayStatics.GetGameInstance`)))
  (for _array_element _persistentheroes
    (bind ((`StartingStatuses_7_FA7A44FD441B281032B5FE8B5F3F9AAA` _startingstatuses) (`UniqueID_53_2854C97C4349924C1E5F7B922ADBA3AE` _uniqueid) (`StatusLimits_59_A60ADA454B18090635BFD49A6D1EDD57` _statuslimits)) (break `/Game/RLDB/Blueprints/Structs/FMinion` _array_element))
    (message `/Game/RLDB/Blueprints/Interfaces/BPI_CardGameInstance.UpdateHeroPersistentHealth` (`GameplayStatics.GetGameInstance`) _uniqueid (`KismetMathLibrary.Min` (+ (`BlueprintMapLibrary.Map_Find` _startingstatuses "/Game/RLDB/Blueprints/Statuses/BP_Status_Health.BP_Status_Health_C") (`local.HealAmount`)) (`BlueprintMapLibrary.Map_Find` _statuslimits "/Game/RLDB/Blueprints/Statuses/BP_Status_Health.BP_Status_Health_C"))))
  (return))

(fn `SetupAndLoadArena`
  (locals (LocalEncounterData :type "DataTable Object Reference"))
  (`|SwitchGameplayTag` (`self.GameplayTag`)
    (:`Default`
      (set `local.LocalEncounterData` "/Game/RLDB/Data/Encounters/DT_CombatEncounters_Normal.DT_CombatEncounters_Normal" :!label _label))
    (:`Encounter.Easy`
      (set `local.LocalEncounterData` "/Game/RLDB/Data/Encounters/DT_CombatEncounters_Easy.DT_CombatEncounters_Easy"))
    (:`Encounter.Normal`
      (goto _label))
    (:`Encounter.Elite`
      (set `local.LocalEncounterData` "/Game/RLDB/Data/Encounters/DT_CombatEncounters_Elite.DT_CombatEncounters_Elite"))
    (:`Encounter.Boss`
      (set `local.LocalEncounterData` "/Game/RLDB/Data/Encounters/DT_CombatEncounters_Boss.DT_CombatEncounters_Boss")))
  (bind _outrownames (`DataTableFunctionLibrary.GetDataTableRowNames` (`local.LocalEncounterData`)))
  (bind _returnvalue (`|GetDataTableRow` (`local.LocalEncounterData`) (`KismetArrayLibrary.Array_Random` _outrownames))
    (:`then`
      (message `/Game/RLDB/Blueprints/Interfaces/BPI_CardGameInstance.SetCurrentEncounterInInstance` (`GameplayStatics.GetGameInstance`) _returnvalue)
      (`GameplayStatics.OpenLevel` (`KismetStringLibrary.Conv_StringToName` (`.Level_9_A25929C34E49E8B28275AF917100AE74` (break `/Game/RLDB/Blueprints/Structs/FEncounter` _returnvalue))))
      (return))
    (:`RowNotFound`
      (return))))

(fn `UserConstructionScript`
  (bind _nodemesh (`self.NodeMesh`))
  (bind (_value _returnvalue) (`BlueprintMapLibrary.Map_Find` (`self.EncounterIcons`) (`self.GameplayTag`)))
  (`self.AddConnectionSplines`)
  (bind _returnvalue_2 (`PrimitiveComponent.CreateDynamicMaterialInstance` _nodemesh 0 (`PrimitiveComponent.GetMaterial` _nodemesh 0) "None"))
  (set `self.NodeMaterial` _returnvalue_2)
  (if _returnvalue
    (`MaterialInstanceDynamic.SetTextureParameterValue` (`self.NodeMaterial`) "Texture" _value)))