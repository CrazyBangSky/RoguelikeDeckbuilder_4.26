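; Node map manager that shows progress through connected BP_Node actors, using the visited-node path stored in the Game Instance.
; It finds the single Origin node, warning if missing or duplicated, and assigns IDs by breadth-first search over node connections.
; Visited IDs are crossed out, and only the last visited node's connections are enabled.
; Selecting any node stops enabling on all nodes and rebuilds the map state.
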(event `self.ReceiveBeginPlay`
  (`self.InitNodeMap`))

(event `UpdateNodeMap`
  (bind _storedpath (`self.StoredPath`))
  (bind _visitednodes (message `/Game/RLDB/Blueprints/Interfaces/BPI_CardGameInstance.GetVisitedMapNodesFromInstance` (`GameplayStatics.GetGameInstance`)))
  (set `self.StoredPath` _visitednodes)
  (`self.FindAndStoreOrigin`)
  (`self.SetUniqueNodeIdsFromOrigin`)
  (for _array_element (`self.StoredPath`)
    (`/Game/RLDB/Blueprints/NodeMap/BP_Node.CrossOut` (`BlueprintMapLibrary.Map_Find` (`self.NodeIds`) _array_element)))
  (for _array_element_2 (`/Game/RLDB/Blueprints/NodeMap/BP_Node.Connections` (`BlueprintMapLibrary.Map_Find` (`self.NodeIds`) (`|GetArrayItem` _storedpath (`KismetArrayLibrary.Array_LastIndex` _storedpath))))
    (`/Game/RLDB/Blueprints/NodeMap/BP_Node.Enable` _array_element_2)))

(event `InitNodeMap`
  (`self.UpdateNodeMap`)
  (bind _outactors (`GameplayStatics.GetAllActorsOfClass` "/Game/RLDB/Blueprints/NodeMap/BP_Node.BP_Node_C"))
  (for _array_element _outactors
    (add `/Game/RLDB/Blueprints/NodeMap/BP_Node.OnNodeSelected` _array_element (delegate `UpdateOnNodeSelected`))))

(event `UpdateOnNodeSelected`
  (params (Node :type "/Game/RLDB/Blueprints/NodeMap/BP_Node Object Reference"))
  (bind _outactors (`GameplayStatics.GetAllActorsOfClass` "/Game/RLDB/Blueprints/NodeMap/BP_Node.BP_Node_C"))
  (for _array_element _outactors
    (`/Game/RLDB/Blueprints/NodeMap/BP_Node.StopEnable` _array_element))
  (`self.UpdateNodeMap`))

(fn `FindAllPathsFromNode`
  (params (OriginNode :type "/Game/RLDB/Blueprints/NodeMap/BP_Node Object Reference"))
  (returns (Paths :type "Map of /Game/RLDB/Blueprints/NodeMap/BP_Node Object Reference to /Game/RLDB/Blueprints/NodeMap/BP_Node Object Reference"))
  (locals (LocalPaths :type "Map of /Game/RLDB/Blueprints/NodeMap/BP_Node Object Reference to /Game/RLDB/Blueprints/NodeMap/BP_Node Object Reference") (LocalOpenNodes :type "Array of /Game/RLDB/Blueprints/NodeMap/BP_Node Object Reference") (LocalOpenNodesChildren :type "Array of /Game/RLDB/Blueprints/NodeMap/BP_Node Object Reference"))
  (`BlueprintMapLibrary.Map_Add` (`local.LocalPaths`) OriginNode)
  (`KismetArrayLibrary.Array_Add` (`local.LocalOpenNodes`) (`local.OriginNode`))
  (while (> (`KismetArrayLibrary.Array_Length` (`local.LocalOpenNodes`)) 0)
    (for _array_element (`local.LocalOpenNodes`)
      (for _array_element_2 (`/Game/RLDB/Blueprints/NodeMap/BP_Node.Connections` _array_element)
        (if (not (`BlueprintMapLibrary.Map_Contains` (`local.LocalPaths`) _array_element_2))
          (`KismetArrayLibrary.Array_Add` (`local.LocalOpenNodesChildren`) _array_element_2)
          (`BlueprintMapLibrary.Map_Add` (`local.LocalPaths`) _array_element_2 _array_element))))
    (set `local.LocalOpenNodes` (`local.LocalOpenNodesChildren`))
    (`KismetArrayLibrary.Array_Clear` (`local.LocalOpenNodesChildren`)))
  (return (`local.LocalPaths`)))

(fn `FindAndStoreOrigin`
  (returns (OriginNode :type "/Game/RLDB/Blueprints/NodeMap/BP_Node Object Reference"))
  (bind _outactors (`GameplayStatics.GetAllActorsOfClass` "/Game/RLDB/Blueprints/NodeMap/BP_Node.BP_Node_C"))
  (for _array_element _outactors
    (if (`/Game/RLDB/Blueprints/NodeMap/BP_Node.bOrigin` _array_element)
      (`/Engine/EditorBlueprintResources/StandardMacros.FlipFlop`
        (:`A`
          (set `self.OriginNode` _array_element))
        (:`B`
          (`KismetSystemLibrary.PrintString` "WARNING: Multiple Origin nodes. Only one node should be set to Origin" true true (struct :`R` 1.0 :`G` 1.0 :`A` 1.0) 99.0)
          (return (`self.OriginNode`))))))
  (bind _originnode (`self.OriginNode`)
    (:`then`
      (return _originnode))
    (:`else`
      (`KismetSystemLibrary.PrintString` "WARNING: No Origin Node found" true true (struct :`R` 1.0 :`G` 1.0 :`A` 1.0) 99.0)
      (return null))))

(fn `SetUniqueNodeIdsFromOrigin`
  (bind _paths (`self.FindAllPathsFromNode` (`self.OriginNode`)))
  (bind _keys (`BlueprintMapLibrary.Map_Keys` _paths))
  (for (_array_element _array_index) _keys
    (`BlueprintMapLibrary.Map_Add` (`self.NodeIds`) _array_index _array_element)
    (set `/Game/RLDB/Blueprints/NodeMap/BP_Node.Id` _array_index _array_element))
  (return))

(fn `UserConstructionScript`)