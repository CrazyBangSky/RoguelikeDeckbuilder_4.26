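; Blueprint function library giving global access to singleton actors in the card game, each found by GetActorOfClass on every call.
; Event functions forward to the dispatcher hub component on BP_GlobalDispatcherHub to bind, unbind, call or queue gameplay-tag events, singly or in batches.
; Other helpers queue delays on BP_ActionManagerRLDB, return BP_CardPlayer, and show screen log messages through that player.
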(fn `BindEventToGlobalDispatcherHub`
  (params (EventHolder :type "Object Object Reference") (EventTag :type "GameplayTag Structure"))
  (bind _returnvalue (`GameplayStatics.GetActorOfClass` (`local.__WorldContext`) "/Game/RLDB/Blueprints/Core/BP_GlobalDispatcherHub.BP_GlobalDispatcherHub_C"))
  (`/Game/RLDB/Blueprints/Core/BP_DispatcherHubComponent.BindEventToHub` (`/Game/RLDB/Blueprints/Core/BP_GlobalDispatcherHub.BP_DispatcherHubComponent` _returnvalue) EventHolder EventTag)
  (return))

(fn `BindMultipleEventsToGlobalDispatcherHub`
  (params (EventHolder :type "Object Object Reference") (EventTags :type "GameplayTagContainer Structure"))
  (bind _returnvalue (`GameplayStatics.GetActorOfClass` (`local.__WorldContext`) "/Game/RLDB/Blueprints/Core/BP_GlobalDispatcherHub.BP_GlobalDispatcherHub_C"))
  (for _array_element (`BlueprintGameplayTagLibrary.BreakGameplayTagContainer` EventTags)
    (`/Game/RLDB/Blueprints/Core/BP_DispatcherHubComponent.BindEventToHub` (`/Game/RLDB/Blueprints/Core/BP_GlobalDispatcherHub.BP_DispatcherHubComponent` _returnvalue) EventHolder _array_element))
  (return))

(fn `CallEventInGlobalDispatcherHub`
  (params (EventTag :type "GameplayTag Structure") (CallingObject :type "Object Object Reference (by ref)") (CallSpecificObject :type "Object Object Reference"))
  (returns (bSuccess :type Boolean))
  (bind _returnvalue (`GameplayStatics.GetActorOfClass` (`local.__WorldContext`) "/Game/RLDB/Blueprints/Core/BP_GlobalDispatcherHub.BP_GlobalDispatcherHub_C"))
  (bind _bsuccess (`/Game/RLDB/Blueprints/Core/BP_DispatcherHubComponent.CallBoundEvents` (`/Game/RLDB/Blueprints/Core/BP_GlobalDispatcherHub.BP_DispatcherHubComponent` _returnvalue) EventTag CallingObject CallSpecificObject false))
  (return _bsuccess))

(fn `CallMultipleEventsInGlobalDispatcherHub`
  (params (EventTags :type "GameplayTagContainer Structure") (CallingObject :type "Object Object Reference (by ref)") (CallSpecificObject :type "Object Object Reference"))
  (returns (bSuccess :type Boolean))
  (bind _returnvalue (`GameplayStatics.GetActorOfClass` (`local.__WorldContext`) "/Game/RLDB/Blueprints/Core/BP_GlobalDispatcherHub.BP_GlobalDispatcherHub_C"))
  (bind _bsuccess (`/Game/RLDB/Blueprints/Core/BP_DispatcherHubComponent.CallMultipleBoundEvents` (`/Game/RLDB/Blueprints/Core/BP_GlobalDispatcherHub.BP_DispatcherHubComponent` _returnvalue) EventTags CallingObject CallSpecificObject true))
  (return _bsuccess))

(fn `GetCardPlayer`
  (returns (CardPlayer :type "/Game/RLDB/Blueprints/Core/BP_CardPlayer Object Reference"))
  (bind _returnvalue (`GameplayStatics.GetActorOfClass` null "/Game/RLDB/Blueprints/Core/BP_CardPlayer.BP_CardPlayer_C"))
  (return _returnvalue))

(fn `GetCardPlayerPure`
  (returns (CardPlayer :type "/Game/RLDB/Blueprints/Core/BP_CardPlayer Object Reference"))
  (bind _returnvalue (`GameplayStatics.GetActorOfClass` null "/Game/RLDB/Blueprints/Core/BP_CardPlayer.BP_CardPlayer_C"))
  (return _returnvalue))

(fn `GetGlobalDispatcherHub`
  (returns (ReturnValue :type "/Game/RLDB/Blueprints/Core/BP_DispatcherHubComponent Object Reference"))
  (bind _returnvalue (`GameplayStatics.GetActorOfClass` (`local.__WorldContext`) "/Game/RLDB/Blueprints/Core/BP_GlobalDispatcherHub.BP_GlobalDispatcherHub_C"))
  (return (`/Game/RLDB/Blueprints/Core/BP_GlobalDispatcherHub.BP_DispatcherHubComponent` _returnvalue)))

(fn `QueueDelay`
  (params (Delay :type "Float (double-precision)"))
  (bind _returnvalue (`GameplayStatics.GetActorOfClass` null "/Game/RLDB/Blueprints/Core/BP_ActionManagerRLDB.BP_ActionManagerRLDB_C"))
  (`/Game/RLDB/Blueprints/Core/BP_ActionManagerRLDB.QueueDelay` _returnvalue Delay)
  (return))

(fn `QueueEventInGlobalDispatcherHub`
  (params (EventTag :type "GameplayTag Structure") (CallingObject :type "Object Object Reference (by ref)") (CallSpecificObject :type "Object Object Reference") (EndDelay :type "Float (double-precision)" :default -1.0))
  (returns (bSuccess :type Boolean))
  (bind _returnvalue (`GameplayStatics.GetActorOfClass` (`local.__WorldContext`) "/Game/RLDB/Blueprints/Core/BP_GlobalDispatcherHub.BP_GlobalDispatcherHub_C"))
  (`/Game/RLDB/Blueprints/Core/BP_DispatcherHubComponent.QueueEvent` (`/Game/RLDB/Blueprints/Core/BP_GlobalDispatcherHub.BP_DispatcherHubComponent` _returnvalue) EventTag CallingObject CallSpecificObject EndDelay)
  (return true))

(fn `SendScreenLogMessage`
  (params (Message :type Text :default "NSLOCTEXT(\"[BCF75373448C419F7DBB4487C3067EF4]\", \"2CA831944F73D9C2033E2692742DEE49\", \"Ivalid Message\")") (Color :type "LinearColor Structure" :default (struct :`R` 1.0 :`A` 1.0)))
  (bind _returnvalue (`GameplayStatics.GetActorOfClass` null "/Game/RLDB/Blueprints/Core/BP_CardPlayer.BP_CardPlayer_C"))
  (`/Game/RLDB/Blueprints/Core/BP_CardPlayer.DisplayScreenLogMessage` _returnvalue Message Color)
  (return))

(fn `UnbindEventFromGlobalDispatcherHub`
  (params (EventHolder :type "Object Object Reference") (EventTag :type "GameplayTag Structure"))
  (bind _returnvalue (`GameplayStatics.GetActorOfClass` (`local.__WorldContext`) "/Game/RLDB/Blueprints/Core/BP_GlobalDispatcherHub.BP_GlobalDispatcherHub_C"))
  (`/Game/RLDB/Blueprints/Core/BP_DispatcherHubComponent.UnbindEventFromHub` (`/Game/RLDB/Blueprints/Core/BP_GlobalDispatcherHub.BP_DispatcherHubComponent` _returnvalue) EventHolder EventTag)
  (return))

(fn `UnbindMultipleEventsFromGlobalDispatcherHub`
  (params (EventHolder :type "Object Object Reference") (EventTags :type "GameplayTagContainer Structure"))
  (bind _returnvalue (`GameplayStatics.GetActorOfClass` (`local.__WorldContext`) "/Game/RLDB/Blueprints/Core/BP_GlobalDispatcherHub.BP_GlobalDispatcherHub_C"))
  (for _array_element (`BlueprintGameplayTagLibrary.BreakGameplayTagContainer` EventTags)
    (`/Game/RLDB/Blueprints/Core/BP_DispatcherHubComponent.UnbindEventFromHub` (`/Game/RLDB/Blueprints/Core/BP_GlobalDispatcherHub.BP_DispatcherHubComponent` _returnvalue) EventHolder _array_element))
  (return))