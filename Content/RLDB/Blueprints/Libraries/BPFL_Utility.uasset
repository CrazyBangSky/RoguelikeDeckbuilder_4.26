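; Blueprint function library of small, independent utility helpers.
; Camera helpers return the first player's camera location or rotate a given actor to look at it.
; Math helpers return the maximum 32-bit integer, lerp 2D vectors per component, and set, add or subtract an integer by a manipulation selector.
; An engine check detects UE5 by parsing the first character of the engine version string.
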(fn `FaceCamera`
  (params (Actor :type "Actor Object Reference"))
  (`Actor.K2_SetActorRotation` Actor (`KismetMathLibrary.FindLookAtRotation` (`Actor.K2_GetActorLocation` Actor) (`PlayerCameraManager.GetCameraLocation` (`GameplayStatics.GetPlayerCameraManager` null))) false)
  (return))

(fn `GetHighestPossibleInteger`
  (returns (HighestPossibleInteger :type Integer))
  (return 2147483647))

(fn `GetManipulatedIntValue`
  (params (Target :type Integer) (Modifier :type Integer) (Manipulation :type "/Game/RLDB/Blueprints/Enums/EManipulation Enum" :default "NewEnumerator2"))
  (returns (Result :type Integer))
  (return (select `/Game/RLDB/Blueprints/Enums/EManipulation` Manipulation :`NewEnumerator2` Modifier :`NewEnumerator0` (+ Target Modifier) :`NewEnumerator1` (- Target Modifier))))

(fn `GetPlayerCameraLocation`
  (returns (Location :type "Vector Structure"))
  (return (`PlayerCameraManager.GetCameraLocation` (`GameplayStatics.GetPlayerCameraManager` null))))

(fn `IsUE5`
  (returns (bTrue :type Boolean))
  (return (== (`KismetStringLibrary.Conv_StringToInt` (`KismetStringLibrary.Left` (`KismetSystemLibrary.GetEngineVersion`) 1)) 5)))

(fn `LerpVector2D`
  (params (A :type "Vector2D Structure") (B :type "Vector2D Structure") (Alpha :type "Float (double-precision)"))
  (returns (ReturnValue :type "Vector2D Structure"))
  (return (`KismetMathLibrary.MakeVector2D` (`KismetMathLibrary.Lerp` A_X B_X Alpha) (`KismetMathLibrary.Lerp` A_Y B_Y Alpha))))