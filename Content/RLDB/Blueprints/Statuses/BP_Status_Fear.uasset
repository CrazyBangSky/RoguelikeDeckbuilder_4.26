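; Fear status for the card game that cuts the damage of its owner's Attack cards by half and loses one stack at the owner's turn start.
; It handles card draw, generate and modify-in-hand events by applying a negative half-damage modifier to qualifying cards.
; Adding stacks fires the modify-in-hand event through the global dispatcher hub for each card in the player's hand.
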(event `self.ReceiveBeginPlay`
  (`/Game/RLDB/Blueprints/Libraries/BPFL_Singletons.BindMultipleEventsToGlobalDispatcherHub` self (struct :`GameplayTags` (struct :`(TagName` "Event.Card.Draw") :`(TagName` "Event.Card.Generate") :`(TagName` "Event.ModifyCardInHand"))))
  (`/Game/RLDB/Blueprints/Core/BP_DispatcherHubComponent.BindEventToHub` (`.ReturnValue` (`self.GetOwnersDispatcherHub`)) self (struct :`TagName` "Event.TurnStart"))
  (`parent.ReceiveBeginPlay`))

(event `/Game/RLDB/Blueprints/Interfaces/BPI_EventHolder.RunEvent`
  (params (EventTag :type "GameplayTag Structure") (CallingObject :type "Object Object Reference (by ref)") (bGlobal :type Boolean))
  (`|SwitchGameplayTag` EventTag
    (:`Event.Card.Draw`
      (bind _asbp_card (cast `/Game/RLDB/Blueprints/Core/BP_Card` CallingObject :!label _label))
      (if (== (`Actor.GetOwner` _asbp_card) (`self.GetOwner`))
        (if (== (`/Game/RLDB/Blueprints/Core/BP_Card.Type` _asbp_card) (struct :`TagName` "Effect.Attack"))
          (bind (_bsuccess _attackdamage) (`/Game/RLDB/Blueprints/Core/BP_Card.GetCardAttackDamage` _asbp_card))
          (if _bsuccess
            (`/Game/RLDB/Blueprints/Core/BP_Card.ModifyCardAttackDamage` _asbp_card (* (/ _attackdamage 2) -1) "NewEnumerator0")))))
    (:`Event.Card.Generate`
      (goto _label))
    (:`Event.ModifyCardInHand`
      (goto _label))
    (:`Event.TurnStart`
      (if (== CallingObject (`self.GetOwner`))
        (`self.SubtractStatusValue` 1)))))

(fn `AddStatusValue`
  (params (Amount :type Integer) (bShowSplashNumber :type Boolean) (bShowSplashIcon :type Boolean) (bRefreshAppearance :type Boolean))
  (returns (NewValue :type Integer))
  (bind _newvalue (`parent.AddStatusValue` Amount bShowSplashNumber bShowSplashIcon false))
  (bind _cardplayer (`/Game/RLDB/Blueprints/Libraries/BPFL_Singletons.GetCardPlayer`))
  (for _array_element (`/Game/RLDB/Blueprints/Piles/BP_PileComponent.Cards` (`Actor.GetComponentByClass` _cardplayer "/Game/RLDB/Blueprints/Piles/BP_PileComponent_Hand.BP_PileComponent_Hand_C"))
    (`/Game/RLDB/Blueprints/Libraries/BPFL_Singletons.CallEventInGlobalDispatcherHub` (struct :`TagName` "Event.ModifyCardInHand") _array_element))
  (return _newvalue))