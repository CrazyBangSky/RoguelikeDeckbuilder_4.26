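; Poisoned status effect that damages its owner at turn start.
; It binds to the owner's dispatcher hub for the TurnStart event and, when the owner is the caller, subtracts its status value from the owner's Health status with a splash number.
; If still valid afterward, it decrements its own value by one and spawns a SimpleAnim action that plays a flinch on the owner's puppet.
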(event `self.ReceiveBeginPlay`
  (`parent.ReceiveBeginPlay`)
  (`/Game/RLDB/Blueprints/Core/BP_DispatcherHubComponent.BindEventToHub` (`.ReturnValue` (`self.GetOwnersDispatcherHub`)) self (struct :`TagName` "Event.TurnStart")))

(event `/Game/RLDB/Blueprints/Interfaces/BPI_EventHolder.RunEvent`
  (params (EventTag :type "GameplayTag Structure") (CallingObject :type "Object Object Reference (by ref)") (bGlobal :type Boolean))
  (`|SwitchGameplayTag` EventTag
    (:`Event.TurnStart`
      (if (== CallingObject (`self.GetOwner`))
        (bind _asactor (cast `Actor` CallingObject))
        (bind _returnvalue (`Actor.GetComponentByClass` _asactor "/Game/RLDB/Blueprints/Statuses/BP_Status_Health.BP_Status_Health_C"))
        (`/Engine/EditorBlueprintResources/StandardMacros.IsValid` _returnvalue
          (:`Is Valid`
            (`self.SubtractStatusValue` _returnvalue (`self.StatusValue`) true false)
            (if (`KismetSystemLibrary.IsValid` self)
              (`self.SubtractStatusValue` 1)
              (bind _puppet (message `/Game/RLDB/Blueprints/Interfaces/BPI_CardTarget.GetPuppet` CallingObject))
              (`|SpawnActorFromClass` "/Game/RLDB/Blueprints/CardActions/BP_Action_SimpleAnim.BP_Action_SimpleAnim_C" (`KismetMathLibrary.MakeTransform` (0.0 0.0 0.0)) "AlwaysSpawn" "OverrideRootScale" null _puppet (struct :`TagName` "Anim.Flinch") 1.5 null))))))))