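; BP_Status is a component representing a valued status on its owner, apparently a base class, with a UI indicator and optional stored maximum.
; Add, subtract and set funnel through AddStatusValue, which fires pre/post dispatcher-hub events, spawns a ModifyStatus action for splash feedback, and destroys the component at zero unless CanBeZero.
; A loop guard caps triggers per tick, resetting via zero-length RetriggerableDelay.
; CancelInterruption sets Interrupt true, identically to Interrupt.
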(event `self.ReceiveBeginPlay`
  (if (`self.bMaxable`)
    (`self.GetAndSetMaxValues`))
  (bind _owneruiref (`self.OwnerUiRef`)
    (:`then`
      (bind _statusindicator (message `/Game/RLDB/Blueprints/Interfaces/BPI_StatusWidget.AddStatusIndicator` _owneruiref self (`self.bShowImmediately`)))
      (set `self.StatusIndicator` _statusindicator))
    (:`else`)))

(event `/Game/RLDB/Blueprints/Interfaces/BPI_EventHolder.SetPriority`
  (params (Priority :type "Float (single-precision)"))
  (set `self.Priority` Priority))

(event `UpdateLoopGuard`
  (set `self.CurrentTriggersThisTick` (+ (`self.CurrentTriggersThisTick`) 1))
  (`KismetSystemLibrary.RetriggerableDelay` 0.0)
  (if (not (< (`self.CurrentTriggersThisTick`) (`self.MaxTriggersPerTick`)))
    (`KismetSystemLibrary.PrintString` (`KismetStringLibrary.Concat_StrStr` "WARNING: " (`KismetSystemLibrary.GetDisplayName` self) " hit the max trigger limit of " (`KismetStringLibrary.Conv_IntToString` (`self.MaxTriggersPerTick`))) true true (struct :`R` 1.0 :`G` 1.0 :`A` 1.0) 9.0))
  (set `self.CurrentTriggersThisTick` 0))

(event `/Game/RLDB/Blueprints/Interfaces/BPI_Interrupt.Interrupt`
  (set `self.bInterrupt` true))

(event `/Game/RLDB/Blueprints/Interfaces/BPI_Interrupt.CancelInterruption`
  (set `self.bInterrupt` true))

(fn `AddStatusValue`
  (params (Amount :type Integer) (bShowSplashNumber :type Boolean) (bShowSplashIcon :type Boolean) (bRefreshAppearance :type Boolean))
  (returns (NewValue :type Integer))
  (locals (LocalOldStatusValue :type Integer :default 0) (LocalSplashIconDelay :type "Float (double-precision)" :default 0.3))
  (bind _friendlyname (`self.FriendlyName`))
  (bind _returnvalue (`KismetStringLibrary.Conv_IntToString` (`KismetMathLibrary.Abs_Int` (`local.Amount`))))
  (`/Game/RLDB/Blueprints/Core/BP_DispatcherHubComponent.CallBoundEvents` (`.ReturnValue` (`self.GetOwnersDispatcherHub`)) (struct :`TagName` "Event.PreModifyStatus") self null true)
  (set `self.IncomingStatusChange` (`local.Amount`))
  (set `local.LocalOldStatusValue` (`self.StatusValue`))
  (set `self.StatusValue` (`KismetMathLibrary.Max` (+ Amount (`self.StatusValue`))))
  (`|SpawnActorFromClass` "/Game/RLDB/Blueprints/CardActions/BP_Action_ModifyStatus.BP_Action_ModifyStatus_C" (`KismetMathLibrary.MakeTransform` (0.0 0.0 0.0)) "AlwaysSpawn" "OverrideRootScale" null self (`self.StatusValue`) (`local.bShowSplashIcon`) (and (`local.bShowSplashNumber`) (or (!= (`local.Amount`) 0) (`self.bCanBeZero`))) (select `bool` (`local.bShowSplashNumber`) :`true` (select `bool` (`self.bCanBeZero`) :`false` (`KismetTextLibrary.Conv_StringToText` (select `bool` (`KismetTextLibrary.TextIsEmpty` _friendlyname) :`false` (`KismetStringLibrary.Concat_StrStr` (`KismetTextLibrary.Conv_TextToString` _friendlyname) " " _returnvalue) :`true` _returnvalue)) :`true` (`self.FriendlyName`))) (`local.bRefreshAppearance`) "" (`KismetMathLibrary.SelectFloat` (`local.LocalSplashIconDelay`) -1.0 (`local.bShowSplashIcon`)) null)
  (`/Game/RLDB/Blueprints/Core/BP_DispatcherHubComponent.CallBoundEvents` (`.ReturnValue` (`self.GetOwnersDispatcherHub`)) (struct :`TagName` "Event.PostModifyStatus") self null true)
  (if (or (> (`self.StatusValue`) 0) (`self.bCanBeZero`))
    (return (`self.StatusValue`))
    (else
      (`self.K2_DestroyComponent`)
      (return 0))))

(fn `CheckLoopGuard`
  (returns (bBelowLimit :type Boolean))
  (`self.UpdateLoopGuard`)
  (return (<= (`self.CurrentTriggersThisTick`) (`self.MaxTriggersPerTick`))))

(fn `GetAndSetMaxValues`
  (bind (_bvalid _max) (message `/Game/RLDB/Blueprints/Interfaces/BPI_CardTarget.GetStatusMax` (`self.GetOwner`) (`GameplayStatics.GetObjectClass` self)))
  (if _bvalid
    (set `self.MaxValue` _max)
    (return)
    (else
      (set `self.MaxValue` (`self.StatusValue`))
      (message `/Game/RLDB/Blueprints/Interfaces/BPI_CardTarget.SetStatusMax` (`self.GetOwner`) (`GameplayStatics.GetObjectClass` self) (`self.MaxValue`))
      (return))))

(fn `GetFriendlyName`
  (returns (FriendlyName :type Text))
  (return (`self.FriendlyName`)))

(fn `GetOwnersDispatcherHub`
  (returns (bValid :type Boolean) (ReturnValue :type "/Game/RLDB/Blueprints/Core/BP_DispatcherHubComponent Object Reference"))
  (bind _returnvalue (`Actor.GetComponentByClass` (`self.GetOwner`) "/Game/RLDB/Blueprints/Core/BP_DispatcherHubComponent.BP_DispatcherHubComponent_C"))
  (bind _returnvalue_2 (`KismetSystemLibrary.IsValid` _returnvalue))
  (if _returnvalue_2
    (return _returnvalue_2 _returnvalue)
    (else
      (return false null))))

(fn `GetPriority`
  (returns (Priority :type "Float (double-precision)"))
  (return (`self.Priority`)))

(fn `MakeAppearanceStruct`
  (returns (StatusAppearance :type "/Game/RLDB/Blueprints/Structs/FStatusAppearance Structure"))
  (return (make `/Game/RLDB/Blueprints/Structs/FStatusAppearance` (`self.StatusValue`) (`self.Icon`) (`self.Tint`) (`self.SlotType`) (`self.TextAlignment`) (`self.Tooltips`) (`self.FriendlyName`))))

(fn `SetStatusValue`
  (params (Amount :type Integer) (bShowSplashNumber :type Boolean) (bShowSplashIcon :type Boolean))
  (returns (NewValue :type Integer))
  (locals (LocalOldStatusValue :type Integer :default 0))
  (bind _newvalue (`self.AddStatusValue` (- Amount (`self.StatusValue`)) bShowSplashNumber bShowSplashIcon))
  (return _newvalue))

(fn `SubtractStatusValue`
  (params (Amount :type Integer) (bShowSplashNumber :type Boolean) (bShowSplashIcon :type Boolean))
  (returns (NewValue :type Integer))
  (locals (LocalOldStatusValue :type Integer :default 0))
  (bind _newvalue (`self.AddStatusValue` (* Amount -1) bShowSplashNumber bShowSplashIcon))
  (return _newvalue))