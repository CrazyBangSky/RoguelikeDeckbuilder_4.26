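; BP_Status_HandSizeArmor is a card-game status that grants its owner armor based on the player's hand size.
; On BeginPlay it registers with the card player's dispatcher hub for the turn-end event.
; When the event runs, it counts the cards in the hand pile and, if any remain, adds that amount of BP_Status_Armor to the owner with a splash.
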(event `self.ReceiveBeginPlay`
  (`parent.ReceiveBeginPlay`)
  (bind _cardplayer (`/Game/RLDB/Blueprints/Libraries/BPFL_Singletons.GetCardPlayer`))
  (bind _bp_dispatcherhubcomponent (`/Game/RLDB/Blueprints/Core/BP_CardPlayer.BP_DispatcherHubComponent` _cardplayer)
    (:`then`
      (`/Game/RLDB/Blueprints/Core/BP_DispatcherHubComponent.BindEventToHub` _bp_dispatcherhubcomponent self (struct :`TagName` "Event.TurnEnd")))
    (:`else`)))

(event `/Game/RLDB/Blueprints/Interfaces/BPI_EventHolder.RunEvent`
  (params (EventTag :type "GameplayTag Structure") (CallingObject :type "Object Object Reference (by ref)") (bGlobal :type Boolean))
  (`|SwitchGameplayTag` EventTag
    (:`Event.TurnEnd`
      (bind _cardplayer (`/Game/RLDB/Blueprints/Libraries/BPFL_Singletons.GetCardPlayer`))
      (bind _returnvalue (`KismetArrayLibrary.Array_Length` (`/Game/RLDB/Blueprints/Piles/BP_PileComponent.Cards` (`Actor.GetComponentByClass` _cardplayer "/Game/RLDB/Blueprints/Piles/BP_PileComponent_Hand.BP_PileComponent_Hand_C"))))
      (if (> _returnvalue 0)
        (message `/Game/RLDB/Blueprints/Interfaces/BPI_CardTarget.AddToStatus` (`self.GetOwner`) "/Game/RLDB/Blueprints/Statuses/BP_Status_Armor.BP_Status_Armor_C" _returnvalue true)))))