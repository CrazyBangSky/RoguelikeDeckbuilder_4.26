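; Status component that refreshes a card player's mana at turn start, using its own status value as the amount.
; On BeginPlay it binds itself to the turn start event through its owner's dispatcher hub.
; When run, it casts the calling object to BP_CardPlayer and, if a BP_Status_Mana component exists, sets that status to this value without splash number or icon.
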(event `self.ReceiveBeginPlay`
  (`parent.ReceiveBeginPlay`)
  (`/Game/RLDB/Blueprints/Core/BP_DispatcherHubComponent.BindMultipleEventsToHub` (`.ReturnValue` (`self.GetOwnersDispatcherHub`)) self (struct :`GameplayTags` (struct :`(TagName` "Event.TurnStart")))))

(event `/Game/RLDB/Blueprints/Interfaces/BPI_EventHolder.RunEvent`
  (params (EventTag :type "GameplayTag Structure") (CallingObject :type "Object Object Reference (by ref)") (bGlobal :type Boolean))
  (bind _asbp_card_player (cast `/Game/RLDB/Blueprints/Core/BP_CardPlayer` CallingObject))
  (bind _returnvalue (`Actor.GetComponentByClass` _asbp_card_player "/Game/RLDB/Blueprints/Statuses/BP_Status_Mana.BP_Status_Mana_C"))
  (if (`KismetSystemLibrary.IsValid` _returnvalue)
    (`|SwitchGameplayTag` EventTag
      (:`Event.TurnStart`
        (`self.SetStatusValue` _returnvalue (`self.StatusValue`) false false)))))