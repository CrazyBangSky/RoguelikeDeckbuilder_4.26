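; Card status component that changes the owning card's mana cost by its status value, clamped at zero.
; On BeginPlay it caches the owning BP_Card, binds to the hand-modify event on the global dispatcher hub and applies the change.
; Each hand-modify event for that card adds the value to the current cost again and signals the card changed.
; A discard branch destroys the component, though this graph does not bind that event.
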(event `self.ReceiveBeginPlay`
  (`parent.ReceiveBeginPlay`)
  (bind _asbp_card (cast `/Game/RLDB/Blueprints/Core/BP_Card` (`self.GetOwner`)))
  (set `self.OwningCard` _asbp_card)
  (`/Game/RLDB/Blueprints/Libraries/BPFL_Singletons.BindMultipleEventsToGlobalDispatcherHub` self (struct :`GameplayTags` (struct :`(TagName` "Event.ModifyCardInHand") :`(TagName` "Event.Card.Discard"))))
  (`self.ModifyCost`))

(event `ModifyCost`
  (`/Game/RLDB/Blueprints/Core/BP_Card.SetCardUseCosts` (`self.OwningCard`) "NewEnumerator0" (`|MakeMap` "/Game/RLDB/Blueprints/Statuses/BP_Status_Mana.BP_Status_Mana_C" (`KismetMathLibrary.Max` (+ (`BlueprintMapLibrary.Map_Find` (`/Game/RLDB/Blueprints/Core/BP_Card.GetCardUseCosts` (`self.OwningCard`) "NewEnumerator0") "/Game/RLDB/Blueprints/Statuses/BP_Status_Mana.BP_Status_Mana_C") (`self.StatusValue`))) :!type "/Game/RLDB/Blueprints/Statuses/BP_Status Class Reference"))
  (`/Game/RLDB/Blueprints/Core/BP_Card.OnThisCardModified` (`self.OwningCard`)))

(event `/Game/RLDB/Blueprints/Interfaces/BPI_EventHolder.RunEvent`
  (params (EventTag :type "GameplayTag Structure") (CallingObject :type "Object Object Reference (by ref)") (bGlobal :type Boolean))
  (if (== CallingObject (`self.OwningCard`))
    (`|SwitchGameplayTag` EventTag
      (:`Event.ModifyCardInHand`
        (`self.ModifyCost`))
      (:`Event.Card.Discard`
        (`self.K2_DestroyComponent`)))))