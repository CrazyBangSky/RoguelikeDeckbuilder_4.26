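; Card status that makes its owning card cheaper in mana as cards are played while it sits in the player's hand.
; Each pre-play event adds StatusValue to a running reduction, despite the ManaReduceOnDraw name.
; Pre-play and modify-in-hand events rewrite the mana cost from a second cost set minus that reduction, floored at zero.
; The reduction resets on the card's own discard or any event received outside the hand.
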(event `self.ReceiveBeginPlay`
  (`parent.ReceiveBeginPlay`)
  (`/Game/RLDB/Blueprints/Libraries/BPFL_Singletons.BindMultipleEventsToGlobalDispatcherHub` self (struct :`GameplayTags` (struct :`(TagName` "Event.PrePlayCard") :`(TagName` "Event.ModifyCardInHand") :`(TagName` "Event.Card.Discard") :`(TagName` "Event.TurnStart")))))

(event `/Game/RLDB/Blueprints/Interfaces/BPI_EventHolder.RunEvent`
  (params (EventTag :type "GameplayTag Structure") (CallingObject :type "Object Object Reference (by ref)") (bGlobal :type Boolean))
  (bind _asbp_card (cast `/Game/RLDB/Blueprints/Core/BP_Card` (`self.GetOwner`) :!pure true))
  (if (`KismetArrayLibrary.Array_Contains` (`/Game/RLDB/Blueprints/Piles/BP_PileComponent.Cards` (`Actor.GetComponentByClass` (`/Game/RLDB/Blueprints/Libraries/BPFL_Singletons.GetCardPlayerPure`) "/Game/RLDB/Blueprints/Piles/BP_PileComponent_Hand.BP_PileComponent_Hand_C")) (cast `/Game/RLDB/Blueprints/Core/BP_Card` (`self.GetOwner`) :!pure true))
    (`|SwitchGameplayTag` EventTag
      (:`Event.PrePlayCard`
        (set `self.CurrentModification` (+ (`self.CurrentModification`) (`self.StatusValue`)))
        (`/Game/RLDB/Blueprints/Core/BP_Card.SetCardUseCosts` _asbp_card "NewEnumerator0" (`|MakeMap` "/Game/RLDB/Blueprints/Statuses/BP_Status_Mana.BP_Status_Mana_C" (`KismetMathLibrary.Max` (- (`BlueprintMapLibrary.Map_Find` (`/Game/RLDB/Blueprints/Core/BP_Card.GetCardUseCosts` _asbp_card "NewEnumerator1") "/Game/RLDB/Blueprints/Statuses/BP_Status_Mana.BP_Status_Mana_C") (`self.CurrentModification`))) :!type "/Game/RLDB/Blueprints/Statuses/BP_Status Class Reference") :!label _label)
        (`/Game/RLDB/Blueprints/Core/BP_Card.OnThisCardModified` (cast `/Game/RLDB/Blueprints/Core/BP_Card` (`self.GetOwner`) :!pure true)))
      (:`Event.ModifyCardInHand`
        (goto _label))
      (:`Event.Card.Discard`
        (if (== CallingObject (`self.GetOwner`))
          (set `self.CurrentModification` 0))))
    (else
      (`|SwitchGameplayTag` EventTag
        (:`Event.TurnStart`
          (set `self.CurrentModification` 0))))))