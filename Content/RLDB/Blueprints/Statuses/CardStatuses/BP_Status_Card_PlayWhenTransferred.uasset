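; Card status that automatically plays its owning card when the card is transferred to a matching pile.
; On BeginPlay it binds to the card's transfer event; the handler, despite its ResetCostOnDiscard name, checks the target pile for an exact match in its GameplayTags.
; On a match it queues delays and an AutoPlay event, fires Card.Generate immediately, then attempts to use the card without targets, keeping playability checks and consequences.
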(event `self.ReceiveBeginPlay`
  (`parent.ReceiveBeginPlay`)
  (add `/Game/RLDB/Blueprints/Core/BP_Card.OnThisCardTransferred` (cast `/Game/RLDB/Blueprints/Core/BP_Card` (`self.GetOwner`) :!pure true) (delegate `ResetCostOnDiscard`)))

(event `ResetCostOnDiscard`
  (params (TargetPileTag :type "GameplayTag Structure"))
  (if (`BlueprintGameplayTagLibrary.HasTag` (`self.GameplayTags`) TargetPileTag true)
    (`/Game/RLDB/Blueprints/Libraries/BPFL_Singletons.QueueDelay` 0.4)
    (`/Game/RLDB/Blueprints/Libraries/BPFL_Singletons.QueueEventInGlobalDispatcherHub` (struct :`TagName` "Event.Action.AutoPlay") (`self.GetOwner`) null 1.0)
    (`/Game/RLDB/Blueprints/Libraries/BPFL_Singletons.CallEventInGlobalDispatcherHub` (struct :`TagName` "Event.Card.Generate") (cast `/Game/RLDB/Blueprints/Core/BP_Card` (`self.GetOwner`) :!pure true))
    (`/Game/RLDB/Blueprints/Core/BP_Card.AttemptUseCard` (cast `/Game/RLDB/Blueprints/Core/BP_Card` (`self.GetOwner`) :!pure true) (`self.EmptyArray`) false false)
    (`/Game/RLDB/Blueprints/Libraries/BPFL_Singletons.QueueDelay` 1.0)))