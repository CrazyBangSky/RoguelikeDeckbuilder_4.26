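; BP_Status_Health is the health status for minions, handling damage, death and reaction animations.
; AddStatusValue fires pre- and post-damage events through the owner's dispatcher hub around the parent change, exposing IncomingStatusChange beforehand, presumably so listeners can modify it.
; It spawns a puppet animation action for die, flinch or block depending on the result.
; A minion at zero health is flagged dead and, after damage, removed from the game.
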(fn `AddStatusValue`
  (params (Amount :type Integer) (bShowSplashNumber :type Boolean) (bShowSplashIcon :type Boolean) (bRefreshAppearance :type Boolean))
  (returns (NewValue :type Integer))
  (set `self.IncomingStatusChange` (`local.Amount`))
  (if (< Amount 0)
    (`/Game/RLDB/Blueprints/Core/BP_DispatcherHubComponent.CallBoundEvents` (`.ReturnValue` (`self.GetOwnersDispatcherHub`)) (struct :`TagName` "Event.PreTakeDamage") self null true) ; Generic one for all statuses?
  )
  (bind _newvalue (`parent.AddStatusValue` (`self.IncomingStatusChange`) (`local.bShowSplashNumber`) (`local.bShowSplashIcon`) false))
  (bind _returnvalue (<= _newvalue 0))
  (if _returnvalue
    (set `/Game/RLDB/Blueprints/Core/BP_Minion.bDead` true (cast `/Game/RLDB/Blueprints/Core/BP_Minion` (`self.GetOwner`) :!pure true)))
  (`|SpawnActorFromClass` "/Game/RLDB/Blueprints/CardActions/BP_Action_SimpleAnim.BP_Action_SimpleAnim_C" (`KismetMathLibrary.MakeTransform` (0.0 0.0 0.0)) "AlwaysSpawn" "OverrideRootScale" null (`/Game/RLDB/Blueprints/Core/BP_Minion.Puppet` (cast `/Game/RLDB/Blueprints/Core/BP_Minion` (`self.GetOwner`) :!pure true)) (select `bool` _returnvalue :`false` (select `bool` (!= (`self.IncomingStatusChange`) 0) :`false` (struct :`TagName` "Anim.Block") :`true` (struct :`TagName` "Anim.Flinch") :!type "GameplayTag Structure") :`true` (struct :`TagName` "Anim.Die")) -1.0 null)
  (if (< (`local.Amount`) 0)
    (`/Game/RLDB/Blueprints/Core/BP_DispatcherHubComponent.CallBoundEvents` (`.ReturnValue` (`self.GetOwnersDispatcherHub`)) (struct :`TagName` "Event.PostTakeDamage") self null true)
    (if (<= (`self.StatusValue`) 0)
      (bind _asbp_minion (cast `/Game/RLDB/Blueprints/Core/BP_Minion` (`self.GetOwner`)))
      (`/Game/RLDB/Blueprints/Core/BP_Minion.RemoveFromGame` _asbp_minion)))
  (return (`self.StatusValue`)))