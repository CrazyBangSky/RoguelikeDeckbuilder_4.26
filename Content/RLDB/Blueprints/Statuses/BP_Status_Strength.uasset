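; Strength status effect for the card game that modifies the attack damage of its owner's attack cards by the status value.
; It binds to the global dispatcher's card draw event, and its event handler also accepts generate and modify-in-hand tags.
; The handler checks for the attack tag and matching owner before modifying damage.
; Adding status value calls the parent, then broadcasts a modify event for each card in the player's hand.
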(event `self.ReceiveBeginPlay`
  (`/Game/RLDB/Blueprints/Libraries/BPFL_Singletons.BindMultipleEventsToGlobalDispatcherHub` self (struct :`GameplayTags` (struct :`(TagName` "Event.Card.Draw") :`(TagName` "Event.Card.Generate") :`(TagName` "Event.ModifyCardInHand"))))
  (`parent.ReceiveBeginPlay`))

(event `/Game/RLDB/Blueprints/Interfaces/BPI_EventHolder.RunEvent`
  (params (EventTag :type "GameplayTag Structure") (CallingObject :type "Object Object Reference (by ref)") (bGlobal :type Boolean))
  (`|SwitchGameplayTag` EventTag
    (:`Event.Card.Draw`
      _)
    (:`Event.Card.Generate`
      _)
    (:`Event.ModifyCardInHand`
      _))
  (bind _asbp_card (cast `/Game/RLDB/Blueprints/Core/BP_Card` CallingObject))
  (if (`BlueprintGameplayTagLibrary.HasTag` (`/Game/RLDB/Blueprints/Core/BP_Card.GetGameplayTags` _asbp_card) (struct :`TagName` "Effect.Attack") true)
    (if (== (`Actor.GetOwner` _asbp_card) (`self.GetOwner`))
      (`/Game/RLDB/Blueprints/Core/BP_Card.ModifyCardAttackDamage` _asbp_card (`self.StatusValue`) "NewEnumerator0"))))

(fn `AddStatusValue`
  (params (Amount :type Integer) (bShowSplashNumber :type Boolean) (bShowSplashIcon :type Boolean) (bRefreshAppearance :type Boolean))
  (returns (NewValue :type Integer))
  (bind _newvalue (`parent.AddStatusValue` Amount bShowSplashNumber bShowSplashIcon false))
  (bind _cardplayer (`/Game/RLDB/Blueprints/Libraries/BPFL_Singletons.GetCardPlayer`))
  (for _array_element (`/Game/RLDB/Blueprints/Piles/BP_PileComponent.Cards` (`Actor.GetComponentByClass` _cardplayer "/Game/RLDB/Blueprints/Piles/BP_PileComponent_Hand.BP_PileComponent_Hand_C"))
    (`/Game/RLDB/Blueprints/Libraries/BPFL_Singletons.CallEventInGlobalDispatcherHub` (struct :`TagName` "Event.ModifyCardInHand") _array_element))
  (return _newvalue))