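; BP_Status_Skittish is a status effect that applies Fear to its owner when that owner takes damage.
; On BeginPlay it binds to the post-damage event on the owner's dispatcher hub.
; A DoOnce gates the reaction before the owner check, then adds Fear equal to the status value with a splash.
; The Turn Start handler resets the gate, though this graph binds only the damage event.
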(event `self.ReceiveBeginPlay`
  (`parent.ReceiveBeginPlay`)
  (`/Game/RLDB/Blueprints/Core/BP_DispatcherHubComponent.BindMultipleEventsToHub` (`.ReturnValue` (`self.GetOwnersDispatcherHub`)) self (struct :`GameplayTags` (struct :`(TagName` "Event.PostTakeDamage") :`(TagName` "Event.TurnStart")))))

(event `/Game/RLDB/Blueprints/Interfaces/BPI_EventHolder.RunEvent`
  (params (EventTag :type "GameplayTag Structure") (CallingObject :type "Object Object Reference (by ref)") (bGlobal :type Boolean))
  (`/Engine/EditorBlueprintResources/StandardMacros.IsValid` CallingObject
    (:`Is Valid`
      (`|SwitchGameplayTag` EventTag
        (:`Event.PostTakeDamage`
          (`/Engine/EditorBlueprintResources/StandardMacros.DoOnce` false :!label _label
            (:`Completed`
              (bind _asactor_component (cast `ActorComponent` CallingObject))
              (if (== (`self.GetOwner` _asactor_component) (`self.GetOwner`))
                (message `/Game/RLDB/Blueprints/Interfaces/BPI_CardTarget.AddToStatus` (`self.GetOwner`) "/Game/RLDB/Blueprints/Statuses/BP_Status_Fear.BP_Status_Fear_C" (`self.StatusValue`) true)))))
        (:`Event.TurnStart`
          (goto _label :!via `Reset`))))))