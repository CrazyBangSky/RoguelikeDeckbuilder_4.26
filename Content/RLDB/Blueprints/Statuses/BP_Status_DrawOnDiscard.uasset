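; BP_Status_DrawOnDiscard is a status Blueprint that makes its card player draw cards when an active discard happens.
; On BeginPlay it binds itself to the global dispatcher hub for the Event.Card.ActiveDiscard tag.
; RunEvent switches on the tag, then calls AttemptDraw on the player's hand pile component once per point of status value, with a minimum of one attempt.
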(event `self.ReceiveBeginPlay`
  (`parent.ReceiveBeginPlay`)
  (`/Game/RLDB/Blueprints/Libraries/BPFL_Singletons.BindEventToGlobalDispatcherHub` self (struct :`TagName` "Event.Card.ActiveDiscard")))

(event `/Game/RLDB/Blueprints/Interfaces/BPI_EventHolder.RunEvent`
  (params (EventTag :type "GameplayTag Structure") (CallingObject :type "Object Object Reference (by ref)") (bGlobal :type Boolean))
  (`|SwitchGameplayTag` EventTag
    (:`Event.Card.ActiveDiscard`
      (bind _cardplayer (`/Game/RLDB/Blueprints/Libraries/BPFL_Singletons.GetCardPlayer`))
      (for _ (range (+ (`KismetMathLibrary.Max` (- (`self.StatusValue`) 1)) 1))
        (`/Game/RLDB/Blueprints/Piles/BP_PileComponent_Hand.AttemptDraw` (`/Game/RLDB/Blueprints/Core/BP_CardPlayer.BP_PileComponent_Hand` _cardplayer))))))