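; Venomous status Blueprint that applies Poisoned to others who take damage while its owner attacks.
; BeginPlay binds to PreAttack on the owner's dispatcher hub and PostTakeDamage on the global hub.
; A gate opened by PreAttack and closed by PostAttack filters damage events to the attack window.
; Damaged non-owner Health statuses queue a splash delay, then their owners receive Poisoned equal to this status's value.
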(event `self.ReceiveBeginPlay`
  (`parent.ReceiveBeginPlay`)
  (`/Game/RLDB/Blueprints/Core/BP_DispatcherHubComponent.BindMultipleEventsToHub` (`.ReturnValue` (`self.GetOwnersDispatcherHub`)) self (struct :`GameplayTags` (struct :`(TagName` "Event.PreAttack") :`(TagName` "Event.PostAttack"))))
  (`/Game/RLDB/Blueprints/Libraries/BPFL_Singletons.BindEventToGlobalDispatcherHub` self (struct :`TagName` "Event.PostTakeDamage")))

(event `/Game/RLDB/Blueprints/Interfaces/BPI_EventHolder.RunEvent`
  (params (EventTag :type "GameplayTag Structure") (CallingObject :type "Object Object Reference (by ref)") (bGlobal :type Boolean))
  (`|SwitchGameplayTag` EventTag
    (:`Event.PostTakeDamage`
      (`/Engine/EditorBlueprintResources/StandardMacros.Gate` true :!label _label
        (:`Exit`
          (bind _asbp_status_health (cast `/Game/RLDB/Blueprints/Statuses/BP_Status_Health` CallingObject))
          (`/Engine/EditorBlueprintResources/StandardMacros.IsValid` _asbp_status_health
            (:`Is Valid`
              (bind _returnvalue (`self.GetOwner` _asbp_status_health))
              (if (!= _returnvalue (`self.GetOwner`))
                (`/Game/RLDB/Blueprints/Libraries/BPFL_Singletons.QueueDelay` (`self.SplashDelay`))
                (message `/Game/RLDB/Blueprints/Interfaces/BPI_CardTarget.AddToStatus` _returnvalue "/Game/RLDB/Blueprints/Statuses/BP_Status_Poisoned.BP_Status_Poisoned_C" (`self.StatusValue`) true)))))))
    (:`Event.PreAttack`
      (goto _label :!via `Open`))
    (:`Event.PostAttack`
      (goto _label :!via `Close`))))