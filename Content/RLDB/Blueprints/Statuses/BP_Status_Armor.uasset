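; Armor status for a minion in a card game, soaking up incoming attack damage.
; On BeginPlay it registers with its owner's dispatcher hub for the incoming attack event.
; Each attack reduces armor by the card effect's value and lowers that value by the old armor, clamped at zero, showing "Blocked" splash text at zero.
; Its turn start handler resets armor to zero, though this graph does not bind that event.
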(event `self.ReceiveBeginPlay`
  (`parent.ReceiveBeginPlay`)
  (`/Game/RLDB/Blueprints/Core/BP_DispatcherHubComponent.BindMultipleEventsToHub` (`.ReturnValue` (`self.GetOwnersDispatcherHub`)) self (struct :`GameplayTags` (struct :`(TagName` "Event.IncomingAttack") :`(TagName` "Event.TurnStart")))))

(event `/Game/RLDB/Blueprints/Interfaces/BPI_EventHolder.RunEvent`
  (params (EventTag :type "GameplayTag Structure") (CallingObject :type "Object Object Reference (by ref)") (bGlobal :type Boolean))
  ;[0 0 0 0.8] When an incoming attack is directed towards the owning Minion, subtracts the Effect value from the incoming attack and reduces the armor value by the same amount
  (`|SwitchGameplayTag` EventTag
    (:`Event.IncomingAttack`
      (bind _asbp_card_effect (cast `/Game/RLDB/Blueprints/CardEffects/BP_CardEffect` CallingObject))
      (set `self.OldArmor` (`self.StatusValue`))
      (`self.SubtractStatusValue` (`/Game/RLDB/Blueprints/CardEffects/BP_CardEffect.EffectValue` _asbp_card_effect))
      (bind _output_get (set `/Game/RLDB/Blueprints/CardEffects/BP_CardEffect.EffectValue` (`KismetMathLibrary.Max` (- (`/Game/RLDB/Blueprints/CardEffects/BP_CardEffect.EffectValue` _asbp_card_effect) (`self.OldArmor`))) _asbp_card_effect))
      (if (== _output_get 0)
        (bind _puppet (message `/Game/RLDB/Blueprints/Interfaces/BPI_CardTarget.GetPuppet` (`self.GetOwner`)))
        (`|SpawnActorFromClass` "/Game/RLDB/Blueprints/CardActions/BP_Action_SplashText.BP_Action_SplashText_C" (`KismetMathLibrary.MakeTransform` (0.0 0.0 0.0)) "Undefined" "OverrideRootScale" null _puppet "Blocked" (struct :`R` 0.7 :`G` 0.7 :`B` 0.7 :`A` 1.0) -1.0 null)))
    (:`Event.TurnStart`
      (`self.SetStatusValue` 0))))