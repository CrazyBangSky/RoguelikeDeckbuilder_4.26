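; Cursed status effect that doubles damage taken by the owning minion and wears off by one each turn.
; On BeginPlay it binds to the turn-start and pre-take-damage events on the owner's dispatcher hub.
; Pre-take-damage doubles the calling Health status's pending change, intended to apply after damage reduction.
; The owner's turn start silently subtracts one from the status value, with no splash feedback.
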(event `self.ReceiveBeginPlay`
  (`parent.ReceiveBeginPlay`)
  (`/Game/RLDB/Blueprints/Core/BP_DispatcherHubComponent.BindEventToHub` (`.ReturnValue` (`self.GetOwnersDispatcherHub`)) self (struct :`TagName` "Event.TurnStart"))
  (`/Game/RLDB/Blueprints/Core/BP_DispatcherHubComponent.BindEventToHub` (`.ReturnValue` (`self.GetOwnersDispatcherHub`)) self (struct :`TagName` "Event.PreTakeDamage")))

(event `/Game/RLDB/Blueprints/Interfaces/BPI_EventHolder.RunEvent`
  (params (EventTag :type "GameplayTag Structure") (CallingObject :type "Object Object Reference (by ref)") (bGlobal :type Boolean))
  ;[0 0 0] Doubles any damage received to the owning minion, after accounting for any damage reduction. Reduces by 1 each turn.
  (`|SwitchGameplayTag` EventTag
    (:`Event.TurnStart`
      (if (== CallingObject (`self.GetOwner`))
        (`self.SubtractStatusValue` 1)))
    (:`Event.PreTakeDamage`
      (bind _asbp_status_health (cast `/Game/RLDB/Blueprints/Statuses/BP_Status_Health` CallingObject))
      (set `/Game/RLDB/Blueprints/Statuses/BP_Status.IncomingStatusChange` (* (`/Game/RLDB/Blueprints/Statuses/BP_Status.IncomingStatusChange` _asbp_status_health) 2) _asbp_status_health))))