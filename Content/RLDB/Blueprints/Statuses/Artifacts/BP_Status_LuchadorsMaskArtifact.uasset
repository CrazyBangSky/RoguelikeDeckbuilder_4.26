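; Artifact status for the Luchador's Mask that grants Strength to every hero minion once, at the first turn start after it begins play.
; On BeginPlay it registers with the global dispatcher hub for the TurnStart event.
; When the event fires, it unbinds itself, then adds Strength equal to its status value, with a splash, to each BP_Minion tagged Target.Hero.
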(event `self.ReceiveBeginPlay`
  (`parent.ReceiveBeginPlay`)
  (`/Game/RLDB/Blueprints/Libraries/BPFL_Singletons.BindEventToGlobalDispatcherHub` self (struct :`TagName` "Event.TurnStart")))

(event `/Game/RLDB/Blueprints/Interfaces/BPI_EventHolder.RunEvent`
  (params (EventTag :type "GameplayTag Structure") (CallingObject :type "Object Object Reference (by ref)") (bGlobal :type Boolean))
  (`|SwitchGameplayTag` EventTag
    (:`Event.TurnStart`
      (`/Game/RLDB/Blueprints/Libraries/BPFL_Singletons.UnbindEventFromGlobalDispatcherHub` self (struct :`TagName` "Event.TurnStart"))
      (bind _outactors (`GameplayStatics.GetAllActorsOfClass` "/Game/RLDB/Blueprints/Core/BP_Minion.BP_Minion_C"))
      (for _array_element _outactors
        (if (`BlueprintGameplayTagLibrary.HasTag` (`/Game/RLDB/Blueprints/Core/BP_Minion.GetGameplayTags` _array_element) (struct :`TagName` "Target.Hero") true)
          (`/Game/RLDB/Blueprints/Core/BP_Minion.AddToStatus` _array_element "/Game/RLDB/Blueprints/Statuses/BP_Status_Strength.BP_Status_Strength_C" (`self.StatusValue`) true))))))