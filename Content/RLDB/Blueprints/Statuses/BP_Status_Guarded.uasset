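; Guarded status for minions, which halves incoming attack values while the owner's minion track holds more than one minion.
; On BeginPlay it caches the owning BP_Minion and binds to the owner's dispatcher hub for the Event.IncomingAttack gameplay tag.
; When the event runs, it checks the track's minion count and directly halves EffectValue on the calling BP_CardEffect.
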(event `self.ReceiveBeginPlay`
  (`parent.ReceiveBeginPlay`)
  (bind _asbp_minion (cast `/Game/RLDB/Blueprints/Core/BP_Minion` (`self.GetOwner`)))
  (set `self.OwningMinion` _asbp_minion)
  (`/Game/RLDB/Blueprints/Core/BP_DispatcherHubComponent.BindEventToHub` (`.ReturnValue` (`self.GetOwnersDispatcherHub`)) self (struct :`TagName` "Event.IncomingAttack")))

(event `/Game/RLDB/Blueprints/Interfaces/BPI_EventHolder.RunEvent`
  (params (EventTag :type "GameplayTag Structure") (CallingObject :type "Object Object Reference (by ref)") (bGlobal :type Boolean))
  (`|SwitchGameplayTag` EventTag
    (:`Event.IncomingAttack`
      (if (> (`KismetArrayLibrary.Array_Length` (`/Game/RLDB/Blueprints/Core/BP_MinionTrack.Minions` (`/Game/RLDB/Blueprints/Core/BP_Minion.MinionTrack` (`self.OwningMinion`)))) 1)
        (bind _asbp_card_effect (cast `/Game/RLDB/Blueprints/CardEffects/BP_CardEffect` CallingObject))
        (set `/Game/RLDB/Blueprints/CardEffects/BP_CardEffect.EffectValue` (/ (`/Game/RLDB/Blueprints/CardEffects/BP_CardEffect.EffectValue` _asbp_card_effect) 2) _asbp_card_effect)))))