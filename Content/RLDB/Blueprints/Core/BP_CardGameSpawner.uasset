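; BP_CardGameSpawner boots a card battle level on BeginPlay by spawning the actors in SpawnOrderActors in order and sending the current level name for saving.
; It then fills two BP_MinionTrack actors through AddMinionToTrack: the first with persistent heroes from the GameInstance, the second with the current encounter's minions resolved from data table rows.
; Tracks are picked by their GetAllActorsOfClass index, so which side is which depends on actor order.
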(event `self.ReceiveBeginPlay`
  (for _array_element (`self.SpawnOrderActors`)
    (`|SpawnActorFromClass` _array_element (`self.GetTransform`) "AlwaysSpawn" "OverrideRootScale" null null))
  (bind _returnvalue (`GameplayStatics.GetCurrentLevelName` true))
  (message `/Game/RLDB/Blueprints/Interfaces/BPI_CardGameInstance.AttemptSaveGame` (`GameplayStatics.GetGameInstance`) _returnvalue)
  (bind _outactors (`GameplayStatics.GetAllActorsOfClass` "/Game/RLDB/Blueprints/Core/BP_MinionTrack.BP_MinionTrack_C"))
  (bind _persistentheroes (message `/Game/RLDB/Blueprints/Interfaces/BPI_CardGameInstance.GetPersistentHeroesFromInstance` (`GameplayStatics.GetGameInstance`)))
  (for _array_element_2 _persistentheroes
    (bind _output (`|GetArrayItem` _outactors))
    (`/Game/RLDB/Blueprints/Core/BP_MinionTrack.AddMinionToTrack` _output (`KismetArrayLibrary.Array_Length` (`/Game/RLDB/Blueprints/Core/BP_MinionTrack.Minions` _output)) _array_element_2 true))
  (bind _currentencounter (message `/Game/RLDB/Blueprints/Interfaces/BPI_CardGameInstance.GetCurrentEncounterFromInstance` (`GameplayStatics.GetGameInstance`)))
  (for _array_element_3 (`.Minions_10_4F0922FD423311AB44916DAA1B6F80E1` (break `/Game/RLDB/Blueprints/Structs/FEncounter` _currentencounter))
    (bind _returnvalue_2 (`|GetDataTableRow` (break `DataTableRowHandle` _array_element_3) (`.RowName` (break `DataTableRowHandle` _array_element_3)))
      (:`then`
        (bind _output_2 (`|GetArrayItem` _outactors 1))
        (`/Game/RLDB/Blueprints/Core/BP_MinionTrack.AddMinionToTrack` _output_2 (`KismetArrayLibrary.Array_Length` (`/Game/RLDB/Blueprints/Core/BP_MinionTrack.Minions` _output_2)) _returnvalue_2 true)))))

(fn `UserConstructionScript`)