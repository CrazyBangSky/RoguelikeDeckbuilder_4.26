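; Turn manager for the card combat, running initiative-ordered rounds and deciding victory or game over.
; Spawned targets join a sorted initiative list; each turn the fastest remaining actor gets TurnStart, and the manager waits for TurnEnd through the global dispatcher hub.
; Deaths trigger checks for surviving heroes and enemies.
; Victory saves hero health, plays the encounter's reward card, then saves deck and game and loads the node map.
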(event `self.ReceiveBeginPlay`
  ;[0 0 0] Begin Play Setup
  (`/Game/RLDB/Blueprints/Libraries/BPFL_Singletons.BindMultipleEventsToGlobalDispatcherHub` self (struct :`GameplayTags` (struct :`(TagName` "Event.TargetSpawned") :`(TagName` "Event.TurnEnd") :`(TagName` "Event.Death") :`(TagName` "Event.WinGame"))))
  (set `self.bSetupDone` true)
  (`/Game/RLDB/Blueprints/Libraries/BPML_Utility.DelayWhile` (== (`KismetArrayLibrary.Array_Length` (`self.InitiativeSortedActors`)) 0)
    (:`Continue`
      (`KismetSystemLibrary.Delay` 0.0)
      (`/Game/RLDB/Blueprints/Libraries/BPFL_Singletons.CallEventInGlobalDispatcherHub` (struct :`TagName` "Event.GameStart") self)
      (`self.StartNewRound`))))

(event `StartNewRound`
  ;[0 0 0] Start New Round
  (`/Engine/EditorBlueprintResources/StandardMacros.IncrementInt` (`self.CurrentRound`)
    (:`  `
      (set `self.RoundOrderActors` (`self.InitiativeSortedActors`))
      (`self.StartNextObjectTurn`))))

(event `StartNextObjectTurn`
  ;[0 0 0] Start next object turn
  (if (not (`self.bCombatOver`))
    (bind (_bsuccess _fastestactor) (`self.GetRemainingActorWithHighestInitiative`))
    (if _bsuccess
      (bind _output_get (set `self.ActiveActor` _fastestactor))
      (`/Game/RLDB/Blueprints/Core/BP_DispatcherHubComponent.CallBoundEvents` (`self.GetComponentByClass` _output_get "/Game/RLDB/Blueprints/Core/BP_DispatcherHubComponent.BP_DispatcherHubComponent_C") (struct :`TagName` "Event.TurnStart") _output_get null true) ; From here, waits for the actor to call TurnEnd in the global Dispatcher Hub\n(check RunEvent on this graph)
      (else
        (`KismetSystemLibrary.Delay` 0.0)
        (`self.StartNewRound`)))))

(event `EndTurn`
  ;[0 0 0] End Turn
  (bind _activeactor (`self.ActiveActor`)
    (:`then`
      (if (`KismetArrayLibrary.Array_Contains` (`self.RoundOrderActors`) _activeactor)
        (`KismetArrayLibrary.Array_RemoveItem` (`self.RoundOrderActors`) _activeactor)))
    (:`else`
      _))
  (`KismetSystemLibrary.Delay` 0.0)
  (`self.StartNextObjectTurn`))

(event `AddSpawnedActorToInitiative`
  (params (SpawnedActor :type "Actor Object Reference"))
  ;[0 0 0] Add spawned actor to initiative
  (`self.AddActorToInitiative` SpawnedActor (`self.InitiativeSortedActors`))
  (add `self.OnDestroyed` SpawnedActor (delegate `RemoveActorIfDestroyed`))
  (if (== (`self.ActiveActor`) (`/Game/RLDB/Blueprints/Libraries/BPFL_Singletons.GetCardPlayerPure`))
    (`self.AddActorToInitiative` SpawnedActor (`self.RoundOrderActors`))))

(event `/Game/RLDB/Blueprints/Interfaces/BPI_EventHolder.RunEvent`
  (params (EventTag :type "GameplayTag Structure") (CallingObject :type "Object Object Reference (by ref)") (bGlobal :type Boolean))
  (bind _returnvalue (== CallingObject (`self.ActiveActor`)))
  ;[0 0 0] Dispatcher Events
  (`|SwitchGameplayTag` EventTag
    (:`Event.TargetSpawned`
      (bind _asactor (cast `Actor` CallingObject))
      (`self.AddSpawnedActorToInitiative` _asactor))
    (:`Event.TurnEnd`
      (`self.EndTurn`))
    (:`Event.Death`
      (`self.CheckIfCombatShouldEndAfterDeath`)
      (if (not (`self.bCombatOver`))
        (if _returnvalue
          (`KismetSystemLibrary.Delay` 0.0)
          (if _returnvalue
            (`self.EndTurn`)))))
    (:`Event.PostPlayCard`
      (`/Engine/EditorBlueprintResources/StandardMacros.Gate` false :!label _label
        (:`Exit`
          (`self.ExitCombat`))))
    (:`Event.WinGame`
      (`/Game/RLDB/Blueprints/Libraries/BPFL_Singletons.QueueEventInGlobalDispatcherHub` (struct :`TagName` "Event.Action.WinGame") self)
      (goto _label :!via `Close`))))

(event `RemoveActorIfDestroyed` :!signature `self.OnDestroyed`
  (params (DestroyedActor :type "Actor Object Reference"))
  ;[0 0 0] Add spawned actor to initiative
  (`KismetArrayLibrary.Array_RemoveItem` (`self.RoundOrderActors`) DestroyedActor)
  (`KismetArrayLibrary.Array_RemoveItem` (`self.InitiativeSortedActors`) DestroyedActor))

(event `CheckIfCombatShouldEndAfterDeath`
  ;[0 0 0] End game check
  (bind _bremaining (`self.CheckForRemainingMinionsWithTag` (struct :`TagName` "Target.Hero")))
  (if _bremaining
    (bind _bremaining_2 (`self.CheckForRemainingMinionsWithTag` (struct :`TagName` "Target.Enemy")))
    (if (not _bremaining_2)
      (`self.ExecuteCombatVictory`))
    (else
      (`self.ExecuteGameOver`))))

(event `ExecuteCombatVictory`
  (bind _returnvalue (`GameplayStatics.GetGameInstance`))
  ;[0 0 0] End game check
  ;;[0.01106 0.3906 0] Victory
  (set `self.bCombatOver` true)
  (`/Game/RLDB/Blueprints/Libraries/BPFL_Singletons.CallEventInGlobalDispatcherHub` (struct :`TagName` "Event.Victory") self)
  (bind _persistentheroes (message `/Game/RLDB/Blueprints/Interfaces/BPI_CardGameInstance.GetPersistentHeroesFromInstance` (`GameplayStatics.GetGameInstance`)))
  (for _array_element _persistentheroes
    (bind ((`UniqueID_53_2854C97C4349924C1E5F7B922ADBA3AE` _uniqueid)) (break `/Game/RLDB/Blueprints/Structs/FMinion` _array_element))
    (bind (_bisremaining _minion) (`self.FindMinionAmongRemaining` _uniqueid))
    (if _bisremaining
      (bind _returnvalue_2 (`self.GetComponentByClass` _minion "/Game/RLDB/Blueprints/Statuses/BP_Status_Health.BP_Status_Health_C"))
      (if (and (`BlueprintGameplayTagLibrary.HasTag` (`/Game/RLDB/Blueprints/Core/BP_Minion.GetGameplayTags` _minion) (struct :`TagName` "Target.Hero")) (`KismetSystemLibrary.IsValid` _returnvalue_2))
        (message `/Game/RLDB/Blueprints/Interfaces/BPI_CardGameInstance.UpdateHeroPersistentHealth` (`GameplayStatics.GetGameInstance`) (`.UniqueID_53_2854C97C4349924C1E5F7B922ADBA3AE` (break `/Game/RLDB/Blueprints/Structs/FMinion` (`/Game/RLDB/Blueprints/Core/BP_Minion.MinionData` _minion))) (`/Game/RLDB/Blueprints/Statuses/BP_Status.StatusValue` _returnvalue_2)))
      (else
        (message `/Game/RLDB/Blueprints/Interfaces/BPI_CardGameInstance.UpdateHeroPersistentHealth` (`GameplayStatics.GetGameInstance`) _uniqueid 1))))
  (`KismetSystemLibrary.Delay` 0.0)
  (`/Game/RLDB/Blueprints/Libraries/BPFL_Singletons.QueueDelay` 1.5)
  (`/Game/RLDB/Blueprints/Libraries/BPFL_Singletons.BindEventToGlobalDispatcherHub` self (struct :`TagName` "Event.PostPlayCard"))
  (bind _currentencounter (message `/Game/RLDB/Blueprints/Interfaces/BPI_CardGameInstance.GetCurrentEncounterFromInstance` _returnvalue))
  (bind (_bsuccess _mainhero) (message `/Game/RLDB/Blueprints/Interfaces/BPI_CardGameInstance.GetMainHero` _returnvalue))
  (if _bsuccess
    (bind _returnvalue_3 (`|SpawnActorFromClass` "/Game/RLDB/Blueprints/Core/BP_Card.BP_Card_C" (`KismetMathLibrary.MakeTransform` (0.0 0.0 0.0)) "AlwaysSpawn" "OverrideRootScale" _mainhero (`/Game/RLDB/Blueprints/Libraries/BPFL_Card.MakeCardStructFromCardData` (`.Reward_6_44451738477E7D0410BE9FAB5E87AC0F` (break `/Game/RLDB/Blueprints/Structs/FEncounter` _currentencounter))) null))
    (`/Game/RLDB/Blueprints/Core/BP_Card.AttemptUseCard` _returnvalue_3 (`|MakeArray` null :!type "Actor Object Reference") false false)
    (else
      (`self.ExitCombat`))))

(event `ExecuteGameOver`
  ;[0 0 0] End game check
  ;;[0.227 0 0.2552] Game Over
  (set `self.bCombatOver` true)
  (`/Game/RLDB/Blueprints/Libraries/BPFL_Singletons.CallEventInGlobalDispatcherHub` (struct :`TagName` "Event.GameOver") self)
  (`KismetSystemLibrary.Delay` 0.0)
  (`/Game/RLDB/Blueprints/Libraries/BPFL_Singletons.QueueEventInGlobalDispatcherHub` (struct :`TagName` "Event.Action.GameOver") self))

(event `ExitCombat`
  (bind _returnvalue (`GameplayStatics.GetGameInstance`))
  ;[0 0 0] End game check
  ;;[0.1283 0.1615 0.02354] Exit combat
  (bind _cardplayer (`/Game/RLDB/Blueprints/Libraries/BPFL_Singletons.GetCardPlayer`))
  (message `/Game/RLDB/Blueprints/Interfaces/BPI_CardGameInstance.UpdateDeckInInstance` (`GameplayStatics.GetGameInstance`) (`/Game/RLDB/Blueprints/Piles/BP_PileComponent.Cards` (`self.GetComponentByClass` _cardplayer "/Game/RLDB/Blueprints/Piles/BP_PileComponent_Deck.BP_PileComponent_Deck_C")))
  (bind _currentnodemap (message `/Game/RLDB/Blueprints/Interfaces/BPI_CardGameInstance.GetCurrentNodeMapFromInstance` _returnvalue))
  (message `/Game/RLDB/Blueprints/Interfaces/BPI_CardGameInstance.AttemptSaveGame` _returnvalue _currentnodemap)
  (`/Game/RLDB/Blueprints/Libraries/BPFL_Singletons.QueueDelay` 0.5)
  (`|SpawnActorFromClass` "/Game/RLDB/Blueprints/CardActions/BP_Action_LoadMap.BP_Action_LoadMap_C" (`KismetMathLibrary.MakeTransform` (0.0 0.0 0.0)) "AlwaysSpawn" "OverrideRootScale" null _currentnodemap -1.0 null))

(fn `AddActorToInitiative`
  (params (Actor :type "Actor Object Reference") (InitativeArray :type "Array of Actor Object Reference (by ref)"))
  (returns (InitiativeIndex :type Integer))
  (for (_array_element _array_index) InitativeArray
    (bind _initiative (message `/Game/RLDB/Blueprints/Interfaces/BPI_Initiative_RLDB.GetInitiative` _array_element))
    (bind _initiative_2 (message `/Game/RLDB/Blueprints/Interfaces/BPI_Initiative_RLDB.GetInitiative` (`local.Actor`)))
    (if (>= _initiative_2 _initiative)
      (`KismetArrayLibrary.Array_Insert` (`local.InitativeArray`) (`local.Actor`) _array_index)
      (return _array_index)))
  (`KismetArrayLibrary.Array_Add` (`local.InitativeArray`) (`local.Actor`))
  (return 0))

(fn `CheckForRemainingMinionsWithTag`
  (params (Tag :type "GameplayTag Structure"))
  (returns (bRemaining :type Boolean))
  (bind _outactors (`GameplayStatics.GetAllActorsOfClass` "/Game/RLDB/Blueprints/Core/BP_Minion.BP_Minion_C"))
  (for _array_element _outactors
    (if (and (`BlueprintGameplayTagLibrary.HasTag` (`/Game/RLDB/Blueprints/Core/BP_Minion.GetGameplayTags` _array_element) Tag true) (not (`/Game/RLDB/Blueprints/Core/BP_Minion.bDead` _array_element)))
      (return true)))
  (return false))

(fn `FindMinionAmongRemaining`
  (params (MinionUniqueId :type String))
  (returns (bIsRemaining :type Boolean) (Minion :type "/Game/RLDB/Blueprints/Core/BP_Minion Object Reference"))
  (bind _outactors (`GameplayStatics.GetAllActorsOfClass` "/Game/RLDB/Blueprints/Core/BP_Minion.BP_Minion_C"))
  (for _array_element _outactors
    (if (`KismetStringLibrary.EqualEqual_StrStr` (`.UniqueID_53_2854C97C4349924C1E5F7B922ADBA3AE` (break `/Game/RLDB/Blueprints/Structs/FMinion` (`/Game/RLDB/Blueprints/Core/BP_Minion.MinionData` _array_element))) (`local.MinionUniqueId`))
      (return true _array_element)))
  (return false null))

(fn `GetFriendlyName`
  (returns (FriendlyName :type Text))
  (return ""))

(fn `GetPriority`
  (returns (Priority :type "Float (double-precision)"))
  (return 0.0))

(fn `GetRemainingActorWithHighestInitiative`
  (returns (bSuccess :type Boolean) (FastestActor :type "Actor Object Reference"))
  (locals (LocalInitiative :type "Float (double-precision)" :default -999999.0) (LocalFastestActor :type "Actor Object Reference"))
  (bind _localfastestactor (`local.LocalFastestActor`))
  (for _array_element (`self.RoundOrderActors`)
    (bind _initiative (message `/Game/RLDB/Blueprints/Interfaces/BPI_Initiative_RLDB.GetInitiative` _array_element))
    (if (> _initiative (`local.LocalInitiative`))
      (set `local.LocalInitiative` _initiative)
      (set `local.LocalFastestActor` _array_element)))
  (return (`KismetSystemLibrary.IsValid` _localfastestactor) _localfastestactor))

(fn `UserConstructionScript`)