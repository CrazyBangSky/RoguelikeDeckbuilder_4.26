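; Reward manager component that rolls random card and artifact rewards by rarity.
; On BeginPlay it buckets data table rows by Rarity gameplay tag, then removes artifacts the game instance reports from the pool.
; Weighted rolls use custom, default, single-rarity or, for cards, pool-size weights.
; Duplicate cards are swapped for unique ones of that rarity, empty artifact rarities fall through to others, and debug rewards serve as last resort.
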(event `self.ReceiveBeginPlay`
  (`self.GenerateRaritySortedCards`)
  (`self.GenerateRaritySortedArtifacts`)
  (bind _artifacts (message `/Game/RLDB/Blueprints/Interfaces/BPI_CardGameInstance.GetArtifactsFromInstance` (`GameplayStatics.GetGameInstance`)))
  (for _array_element _artifacts
    (`self.RemoveArtifactRewardOption` _array_element)))

(fn `AttemptFindValidUniqueCard`
  (params (CardOptions :type "Array of /Game/RLDB/Blueprints/Structs/FCard Structure") (ChosenCards :type "Array of /Game/RLDB/Blueprints/Structs/FCard Structure") (NonuniqueCardIndex :type Integer))
  (returns (bSuccess :type Boolean) (ValidUniqueCard :type "/Game/RLDB/Blueprints/Structs/FCard Structure"))
  (if (not (`KismetArrayLibrary.Array_Identical` CardOptions ChosenCards))
    (for _index (range (+ (`KismetArrayLibrary.Array_LastIndex` CardOptions) 1))
      (bind _output (`|GetArrayItem` (`local.CardOptions`) (mod (+ _index (`local.NonuniqueCardIndex`)) (`KismetArrayLibrary.Array_Length` (`local.CardOptions`)))))
      (if (not (`KismetArrayLibrary.Array_Contains` (`local.ChosenCards`) _output))
        (return true _output))))
  (return false))

(fn `GenerateRaritySortedArtifacts`
  (returns (RaritySortedArtifacts :type "Map of GameplayTag Structure to /Game/RLDB/Blueprints/Structs/FDataTableRows Structure"))
  (locals (LocalCurrentCardsOfRarity :type "Array of /Game/RLDB/Blueprints/Structs/FCard Structure") (LocalDataRow :type "DataTableRowHandle Structure" :default (struct)) (LocalCurrentArtifactsOfRarity :type "Array of DataTableRowHandle Structure"))
  (bind _returnvalue_gameplaytags (break `GameplayTagContainer` (`BlueprintGameplayTagLibrary.MakeLiteralGameplayTagContainer` (struct :`GameplayTags` (struct :`(TagName` "Rarity.Common") :`(TagName` "Rarity.Epic") :`(TagName` "Rarity.Legendary") :`(TagName` "Rarity.Rare"))))))
  (for _array_element _returnvalue_gameplaytags
    (`BlueprintMapLibrary.Map_Add` (`self.RaritySortedArtifacts`) _array_element))
  (for _array_element_2 (`self.ArtifactTables`)
    (bind _outrownames (`DataTableFunctionLibrary.GetDataTableRowNames` _array_element_2))
    (for _array_element_3 _outrownames
      (bind _output_get (set `local.LocalDataRow` (make `DataTableRowHandle` _array_element_2 _array_element_3)))
      (bind _returnvalue (`|GetDataTableRow` (break `DataTableRowHandle` _output_get) (`.RowName` (break `DataTableRowHandle` _output_get)))
        (:`then`
          (for _array_element_4 (break `GameplayTagContainer` (`.GameplayTags_8_DF9ADDDD4936D0F3EC872485AEA6A35C` (break `/Game/RLDB/Blueprints/Structs/FStatus` _returnvalue)))
            (if (`BlueprintGameplayTagLibrary.MatchesTag` _array_element_4 (struct :`TagName` "Rarity"))
              (bind _output_get_2 (set `local.LocalCurrentArtifactsOfRarity` (break `/Game/RLDB/Blueprints/Structs/FDataTableRows` (`BlueprintMapLibrary.Map_Find` (`self.RaritySortedArtifacts`) _array_element_4))))
              (`KismetArrayLibrary.Array_Add` _output_get_2 (make `DataTableRowHandle` (break `DataTableRowHandle` _output_get) (`.RowName` (break `DataTableRowHandle` _output_get))))
              (`BlueprintMapLibrary.Map_Add` (`self.RaritySortedArtifacts`) _array_element_4 (make `/Game/RLDB/Blueprints/Structs/FDataTableRows` (`local.LocalCurrentArtifactsOfRarity`)))))))))
  (return (`self.RaritySortedArtifacts`)))

(fn `GenerateRaritySortedCards`
  (returns (RaritySortedCards :type "Map of GameplayTag Structure to /Game/RLDB/Blueprints/Structs/FCardStructs Structure"))
  (locals (LocalCurrentCardsOfRarity :type "Array of /Game/RLDB/Blueprints/Structs/FCard Structure") (LocalDataRow :type "DataTableRowHandle Structure" :default (struct)))
  (bind _returnvalue_gameplaytags (break `GameplayTagContainer` (`BlueprintGameplayTagLibrary.MakeLiteralGameplayTagContainer` (struct :`GameplayTags` (struct :`(TagName` "Rarity.Common") :`(TagName` "Rarity.Epic") :`(TagName` "Rarity.Legendary") :`(TagName` "Rarity.Rare"))))))
  (for _array_element _returnvalue_gameplaytags
    (`BlueprintMapLibrary.Map_Add` (`self.RaritySortedCards`) _array_element))
  (bind _rewardtables (message `/Game/RLDB/Blueprints/Interfaces/BPI_CardGameInstance.GetRewardTables` (`GameplayStatics.GetGameInstance`)))
  (for _array_element_2 _rewardtables
    (bind _outrownames (`DataTableFunctionLibrary.GetDataTableRowNames` _array_element_2))
    (for _array_element_3 _outrownames
      (bind _output_get (set `local.LocalDataRow` (make `DataTableRowHandle` _array_element_2 _array_element_3)))
      (bind _returnvalue (`|GetDataTableRow` (break `DataTableRowHandle` _output_get) (`.RowName` (break `DataTableRowHandle` _output_get)))
        (:`then`
          (for _array_element_4 (break `GameplayTagContainer` (`.CardTags_11_D3139088485C66B7F2D8AC86C3BF08B5` (break `/Game/RLDB/Blueprints/Structs/FCard` _returnvalue)))
            (if (`BlueprintGameplayTagLibrary.MatchesTag` _array_element_4 (struct :`TagName` "Rarity"))
              (set `local.LocalCurrentCardsOfRarity` (break `/Game/RLDB/Blueprints/Structs/FCardStructs` (`BlueprintMapLibrary.Map_Find` (`self.RaritySortedCards`) _array_element_4)))
              (bind _structout (setmembers `/Game/RLDB/Blueprints/Structs/FCard` :`StructRef` _returnvalue :`DataRow` (`local.LocalDataRow`)))
              (`KismetArrayLibrary.Array_Add` (`local.LocalCurrentCardsOfRarity`) _structout)
              (`BlueprintMapLibrary.Map_Add` (`self.RaritySortedCards`) _array_element_4 (make `/Game/RLDB/Blueprints/Structs/FCardStructs` (`local.LocalCurrentCardsOfRarity`)))))))))
  (return (`self.RaritySortedCards`)))

(fn `GetRandomArtifactByCustomRarityWeights`
  (params (RarityWeights :type "Map of GameplayTag Structure to Float (double-precision)"))
  (returns (bSuccess :type Boolean) (ArtifactRow :type "DataTableRowHandle Structure") (ArtifactStatus :type "/Game/RLDB/Blueprints/Structs/FStatus Structure"))
  (locals (LocalWeightCount :type "Float (double-precision)") (LocalWeightSum :type "Float (double-precision)") (LocalWeightSelection :type "Float (double-precision)") (LocalRandomArtifact :type "DataTableRowHandle Structure"))
  (bind (_datatable _rowname) (break `DataTableRowHandle` (`local.LocalRandomArtifact`)))
  (bind _keys (`BlueprintMapLibrary.Map_Keys` RarityWeights))
  (for _array_element _keys
    (set `local.LocalWeightSum` (+ (`BlueprintMapLibrary.Map_Find` (`local.RarityWeights`) _array_element) (`local.LocalWeightSum`))))
  (set `local.LocalWeightSelection` (`KismetMathLibrary.RandomFloatInRange` 0.0 (`local.LocalWeightSum`)))
  (bind _keys_2 (`BlueprintMapLibrary.Map_Keys` (`local.RarityWeights`)))
  (for _array_element_2 _keys_2
    (bind _output_get (set `local.LocalWeightCount` (+ (`local.LocalWeightCount`) (`BlueprintMapLibrary.Map_Find` (`local.RarityWeights`) _array_element_2))))
    (if (>= _output_get (`local.LocalWeightSelection`))
      (bind _value (`BlueprintMapLibrary.Map_Find` (`self.RaritySortedArtifacts`) _array_element_2))
      (if (> (`KismetArrayLibrary.Array_Length` (break `/Game/RLDB/Blueprints/Structs/FDataTableRows` _value)) 0)
        (set `local.LocalRandomArtifact` (`KismetArrayLibrary.Array_Random` (break `/Game/RLDB/Blueprints/Structs/FDataTableRows` _value)))
        (bind _returnvalue (`|GetDataTableRow` _datatable _rowname :!label _label)
          (:`then`
            (return true (`local.LocalRandomArtifact`) _returnvalue))
          (:`RowNotFound`
            (return false)))
        (else
          (bind _keys_3 (`BlueprintMapLibrary.Map_Keys` (`local.RarityWeights`)))
          (for _array_element_3 _keys_3
            (bind _value_2 (`BlueprintMapLibrary.Map_Find` (`self.RaritySortedArtifacts`) _array_element_3))
            (if (> (`KismetArrayLibrary.Array_Length` (break `/Game/RLDB/Blueprints/Structs/FDataTableRows` _value_2)) 0)
              (set `local.LocalRandomArtifact` (`KismetArrayLibrary.Array_Random` (break `/Game/RLDB/Blueprints/Structs/FDataTableRows` _value_2)))
              (goto _label)))
          (bind _returnvalue_2 (`|GetDataTableRow` "/Game/RLDB/Data/DT_Artifacts.DT_Artifacts" "Lollipop")
            (:`then`
              (`KismetSystemLibrary.PrintString` "WARNING: No valid artifacts left. Returning debug artifact." true true (struct :`R` 1.0 :`G` 1.0 :`A` 1.0) 9.0)
              (return true (make `DataTableRowHandle` "/Game/RLDB/Data/DT_Artifacts.DT_Artifacts" "Lollipop") _returnvalue_2))
            (:`RowNotFound`
              (`KismetSystemLibrary.PrintString` "WARNING: No valid artifacts left or debug artifact." true true (struct :`R` 1.0 :`G` 1.0 :`A` 1.0) 9.0)
              (return false)))))))
  (`KismetSystemLibrary.PrintString` "WARNING: No valid artifact was found" true true (struct :`R` 1.0 :`G` 1.0 :`A` 1.0) 9.0)
  (return false))

(fn `GetRandomArtifactByDefaultRarityWeights`
  (returns (bSuccess :type Boolean) (ArtifactRow :type "DataTableRowHandle Structure") (ArtifactStatus :type "/Game/RLDB/Blueprints/Structs/FStatus Structure"))
  (locals (LocalWeightCount :type "Float (double-precision)") (LocalWeightSum :type "Float (double-precision)") (LocalWeightSelection :type "Float (double-precision)"))
  (bind (_bsuccess _artifactrow _artifactstatus) (`self.GetRandomArtifactByCustomRarityWeights` (`self.DefaultArtifactRarityWeights`)))
  (return _bsuccess _artifactrow _artifactstatus))

(fn `GetRandomArtifactOfSpecificRarity`
  (params (Rarity :type "GameplayTag Structure"))
  (returns (bSuccess :type Boolean) (ArtifactRow :type "DataTableRowHandle Structure") (ArtifactStatus :type "/Game/RLDB/Blueprints/Structs/FStatus Structure"))
  (locals (LocalWeightCount :type "Float (double-precision)") (LocalWeightSum :type "Float (double-precision)") (LocalWeightSelection :type "Float (double-precision)"))
  (bind (_bsuccess _artifactrow _artifactstatus) (`self.GetRandomArtifactByCustomRarityWeights` (`|MakeMap` Rarity 1.0 :!valuetype "Float (single-precision)")))
  (return _bsuccess _artifactrow _artifactstatus))

(fn `GetRandomCardsByCustomRarityWeights`
  (params (RarityWeights :type "Map of GameplayTag Structure to Float (double-precision)") (Amount :type Integer :default 1))
  (returns (RandomCards :type "Array of /Game/RLDB/Blueprints/Structs/FCard Structure"))
  (locals (LocalWeightCount :type "Float (double-precision)") (LocalWeightSum :type "Float (double-precision)") (LocalWeightSelection :type "Float (double-precision)") (LocalCards :type "Array of /Game/RLDB/Blueprints/Structs/FCard Structure") (LocalCard :type "/Game/RLDB/Blueprints/Structs/FCard Structure"))
  (bind _keys (`BlueprintMapLibrary.Map_Keys` RarityWeights))
  (for _array_element _keys
    (set `local.LocalWeightSum` (+ (`BlueprintMapLibrary.Map_Find` (`local.RarityWeights`) _array_element) (`local.LocalWeightSum`))))
  (for _ (range (`local.Amount`))
    (set `local.LocalWeightSelection` (`KismetMathLibrary.RandomFloatInRange` 0.0 (`local.LocalWeightSum`)))
    (set `local.LocalWeightCount` 0.0)
    (bind _keys_2 (`BlueprintMapLibrary.Map_Keys` (`local.RarityWeights`)))
    (for _array_element_2 _keys_2
      (bind _output_get (set `local.LocalWeightCount` (+ (`local.LocalWeightCount`) (`BlueprintMapLibrary.Map_Find` (`local.RarityWeights`) _array_element_2))))
      (if (>= _output_get (`local.LocalWeightSelection`))
        (`|ExecutionSequence`
          (:`then_0`
            (bind _value (`BlueprintMapLibrary.Map_Find` (`self.RaritySortedCards`) _array_element_2))
            (bind _output_get_2 (set `local.LocalCard` (`KismetArrayLibrary.Array_Random` (break `/Game/RLDB/Blueprints/Structs/FCardStructs` _value))))
            (if (`KismetArrayLibrary.Array_Contains` (`local.LocalCards`) _output_get_2)
              (bind (_bsuccess _validuniquecard) (`self.AttemptFindValidUniqueCard` (break `/Game/RLDB/Blueprints/Structs/FCardStructs` _value) (`local.LocalCards`) (`KismetArrayLibrary.Array_Find` (break `/Game/RLDB/Blueprints/Structs/FCardStructs` _value) (`local.LocalCard`))))
              (if _bsuccess
                (`KismetArrayLibrary.Array_Add` (`local.LocalCards`) _validuniquecard)
                (else
                  (bind _returnvalue (`|GetDataTableRow` "/Game/RLDB/Data/Cards/DT_Cards_Unobtainable.DT_Cards_Unobtainable" "ConsolationPrize")
                    (:`then`
                      (bind _structout (setmembers `/Game/RLDB/Blueprints/Structs/FCard` :`StructRef` _returnvalue :`DataRow` (make `DataTableRowHandle` "/Game/RLDB/Data/Cards/DT_Cards_Unobtainable.DT_Cards_Unobtainable" "ConsolationPrize")))
                      (`KismetArrayLibrary.Array_Add` (`local.LocalCards`) _structout)
                      (`KismetSystemLibrary.PrintString` "WARNING: Not enough valid card options. Returning backup debug card." true true (struct :`R` 1.0 :`G` 1.0 :`A` 1.0) 9.0))
                    (:`RowNotFound`
                      (`KismetSystemLibrary.PrintString` "ERROR: Not enough valid card options, and no valid backup option" true true (struct :`R` 0.995 :`A` 1.0) 99.0)
                      (return (`local.LocalCards`))))))
              (else
                (`KismetArrayLibrary.Array_Add` (`local.LocalCards`) (`local.LocalCard`)))))
          (:`then_1`
            (break))))))
  (return (`local.LocalCards`)))

(fn `GetRandomCardsByDefaultRarityWeights`
  (params (Amount :type Integer :default 1))
  (returns (RandomCards :type "Array of /Game/RLDB/Blueprints/Structs/FCard Structure"))
  (locals (LocalWeightCount :type "Float (double-precision)") (LocalWeightSum :type "Float (double-precision)") (LocalWeightSelection :type "Float (double-precision)"))
  (bind _randomcards (`self.GetRandomCardsByCustomRarityWeights` (`self.DefaultCardRarityWeights`) Amount))
  (return _randomcards))

(fn `GetRandomCardsOfSpecificRarity`
  (params (Rarity :type "GameplayTag Structure") (Amount :type Integer :default 1))
  (returns (RandomCards :type "Array of /Game/RLDB/Blueprints/Structs/FCard Structure"))
  (locals (LocalWeightCount :type "Float (double-precision)") (LocalWeightSum :type "Float (double-precision)") (LocalWeightSelection :type "Float (double-precision)"))
  (bind _randomcards (`self.GetRandomCardsByCustomRarityWeights` (`|MakeMap` Rarity 1.0 :!valuetype "Float (single-precision)") Amount))
  (return _randomcards))

(fn `GetTrueRandomCards`
  (params (Amount :type Integer :default 1))
  (returns (RandomCards :type "Array of /Game/RLDB/Blueprints/Structs/FCard Structure"))
  (locals (LocalWeightCount :type "Float (double-precision)") (LocalWeightSum :type "Float (double-precision)") (LocalWeightSelection :type "Float (double-precision)") (LocalTrueRandomWeights :type "Map of GameplayTag Structure to Float (double-precision)"))
  (bind _keys (`BlueprintMapLibrary.Map_Keys` (`self.RaritySortedCards`)))
  (for _array_element _keys
    (`BlueprintMapLibrary.Map_Add` (`local.LocalTrueRandomWeights`) _array_element (`KismetMathLibrary.Conv_IntToDouble` (`KismetArrayLibrary.Array_Length` (break `/Game/RLDB/Blueprints/Structs/FCardStructs` (`BlueprintMapLibrary.Map_Find` (`self.RaritySortedCards`) _array_element))))))
  (bind _randomcards (`self.GetRandomCardsByCustomRarityWeights` (`local.LocalTrueRandomWeights`) Amount))
  (return _randomcards))

(fn `RemoveArtifactRewardOption`
  (params (Artifact :type "DataTableRowHandle Structure"))
  (locals (LocalArtifactsOfRarity :type "Array of DataTableRowHandle Structure"))
  (bind _returnvalue (`|GetDataTableRow` Artifact_DataTable Artifact_RowName)
    (:`then`
      (for _array_element (break `GameplayTagContainer` (`.GameplayTags_8_DF9ADDDD4936D0F3EC872485AEA6A35C` (break `/Game/RLDB/Blueprints/Structs/FStatus` _returnvalue)))
        (if (`BlueprintGameplayTagLibrary.MatchesTag` _array_element (struct :`TagName` "Rarity"))
          (bind (_value _returnvalue_2) (`BlueprintMapLibrary.Map_Find` (`self.RaritySortedArtifacts`) _array_element))
          (if _returnvalue_2
            (bind _output_get (set `local.LocalArtifactsOfRarity` (break `/Game/RLDB/Blueprints/Structs/FDataTableRows` _value)))
            (`KismetArrayLibrary.Array_RemoveItem` _output_get (`local.Artifact`))
            (`BlueprintMapLibrary.Map_Add` (`self.RaritySortedArtifacts`) _array_element (make `/Game/RLDB/Blueprints/Structs/FDataTableRows` (`local.LocalArtifactsOfRarity`))))))
      (return))))