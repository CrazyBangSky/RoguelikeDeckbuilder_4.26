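; BP_MinionTrack is an ordered lane of minions that spawns them, tracks front and back, and derives initiative from position, favoring the front.
; Slot positions are centered and spaced along the Box's Y extent according to minion count.
; Mid-game additions and minion destruction spawn BP_Action_UpdateTrack actors.
; SlideMinionsToPositions snapshots puppet locations after a retriggerable delay, then timeline-lerps them to their slots.
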(event `self.ReceiveBeginPlay`
  (set `/Game/RLDB/Blueprints/Core/BP_GameplayTagComponent.GameplayTags` (`self.InitialGameplayTags`) (`self.BP_GameplayTagComponent`)))

(event `BindTargetRemoval`
  (params (Target :type "Actor Object Reference"))
  (add `self.OnDestroyed` Target (delegate `RemoveActorIfDestroyed`)))

(event `RemoveActorIfDestroyed` :!signature `self.OnDestroyed`
  (params (DestroyedActor :type "Actor Object Reference"))
  (`KismetArrayLibrary.Array_RemoveItem` (`self.Minions`) (cast `/Game/RLDB/Blueprints/Core/BP_Minion` DestroyedActor :!pure true))
  (`|SpawnActorFromClass` "/Game/RLDB/Blueprints/CardActions/BP_Action_UpdateTrack.BP_Action_UpdateTrack_C" (`KismetMathLibrary.MakeTransform` (0.0 0.0 0.0)) "Undefined" "OverrideRootScale" null self 1.5 -1.0 null))

(event `SlideMinionsToPositions`
  (params (StartDelay :type "Float (double-precision)"))
  (bind _puppetlocationspreslide (`self.PuppetLocationsPreSlide`))
  (`KismetSystemLibrary.RetriggerableDelay` StartDelay)
  (`KismetArrayLibrary.Array_Clear` (`self.PuppetLocationsPreSlide`))
  (for _array_element (`self.Minions`)
    (`/Engine/EditorBlueprintResources/StandardMacros.IsValid` _array_element
      (:`Is Valid`
        (`KismetArrayLibrary.Array_Add` _puppetlocationspreslide (`self.K2_GetActorLocation` (`/Game/RLDB/Blueprints/Core/BP_Minion.Puppet` _array_element))))
      (:`Is Not Valid`
        (`KismetArrayLibrary.Array_Add` _puppetlocationspreslide))))
  (bind (_direction _newtrack_0) (`Timeline|TL_Slide` :!via `PlayFromStart`)
    (:`Update`
      (for (_array_element_2 _array_index) (`self.Minions`)
        (`self.K2_SetActorLocation` (`/Game/RLDB/Blueprints/Core/BP_Minion.Puppet` _array_element_2) (`KismetMathLibrary.VLerp` (`|GetArrayItem` (`self.PuppetLocationsPreSlide`) _array_index) (`self.GetTrackLocationAtIndex` _array_index) _newtrack_0) false false)))))

(fn `AddMinionToTrack`
  (params (Index :type Integer) (MinionData :type "/Game/RLDB/Blueprints/Structs/FMinion Structure") (bSpawnedDuringGameplay :type Boolean))
  (returns (SpawnedTarget :type "/Game/RLDB/Blueprints/Core/BP_Minion Object Reference"))
  (bind _minions (`self.Minions`))
  (if bSpawnedDuringGameplay
    (`|SpawnActorFromClass` "/Game/RLDB/Blueprints/CardActions/BP_Action_UpdateTrack.BP_Action_UpdateTrack_C" (`KismetMathLibrary.MakeTransform` (0.0 0.0 0.0)) "AlwaysSpawn" "OverrideRootScale" null self 0.0 -1.0 null))
  (bind _returnvalue (`|SpawnActorFromClass` "/Game/RLDB/Blueprints/Core/BP_Minion.BP_Minion_C" (`KismetMathLibrary.MakeTransform` (`self.GetTrackLocationAtIndex` (`local.Index`)) (`self.K2_GetActorRotation`)) "AlwaysSpawn" "OverrideRootScale" null self (`local.bSpawnedDuringGameplay`) (`local.MinionData`) null))
  (if (> (`KismetArrayLibrary.Array_Length` _minions) 0)
    (if (`KismetSystemLibrary.IsValid` (`|GetArrayItem` _minions (`local.Index`)))
      (`KismetArrayLibrary.Array_Insert` (`self.Minions`) _returnvalue (`local.Index`))
      (else
        (`KismetArrayLibrary.Array_Set` (`self.Minions`) (`local.Index`) _returnvalue true)))
    (else
      (`KismetArrayLibrary.Array_Add` (`self.Minions`) _returnvalue)))
  (`self.BindTargetRemoval` _returnvalue)
  (return _returnvalue))

(fn `GetBackMinion`
  (returns (bValid :type Boolean) (BackTarget :type "Actor Object Reference") (BackIndex :type Integer))
  (bind _minions (`self.Minions`))
  (bind _returnvalue (`KismetArrayLibrary.Array_LastIndex` _minions))
  (bind _output (`|GetArrayItem` _minions _returnvalue))
  (return (`KismetSystemLibrary.IsValid` _output) _output _returnvalue))

(fn `GetFrontMinion`
  (returns (bValid :type Boolean) (FrontTarget :type "Actor Object Reference") (TargetIndex :type Integer))
  (bind _output (`|GetArrayItem` (`self.Minions`)))
  (return (`KismetSystemLibrary.IsValid` _output) _output 0))

(fn `GetInitiativeFromTrack`
  (params (Minion :type "/Game/RLDB/Blueprints/Core/BP_Minion Object Reference"))
  (returns (Initiative :type "Float (double-precision)"))
  (bind _minions (`self.Minions`))
  (return (+ (`self.InitiativeModifier`) (`KismetMathLibrary.Conv_IntToDouble` (`KismetMathLibrary.Max` (- (`KismetArrayLibrary.Array_LastIndex` _minions) (`KismetArrayLibrary.Array_Find` _minions Minion)))))))

(fn `GetTrackLocationAtIndex`
  (params (TrackIndex :type Integer))
  (returns (ReturnValue :type "Vector Structure"))
  (bind (_returnvalue_x _returnvalue_y) (`KismetMathLibrary.BreakVector` (`self.GetActorScale3D`)))
  (bind (_boxextent_x _boxextent_y) (`KismetMathLibrary.BreakVector` (`BoxComponent.BoxExtent` (`self.Box`))))
  (bind _returnvalue (`KismetMathLibrary.Conv_IntToDouble` (+ (`KismetArrayLibrary.Array_LastIndex` (`self.Minions`)) (`self.ForwardOffset`))))
  (return (`KismetMathLibrary.TransformLocation` (`self.GetTransform`) (`KismetMathLibrary.MakeVector` 0.0 (* (- (`KismetMathLibrary.Conv_IntToDouble` (+ TrackIndex (`self.ForwardOffset`))) (/ _returnvalue 2.0)) (* (* (* (/ 1.0 (+ _returnvalue 2.0)) _boxextent_y) -2.0) _returnvalue_y))))))

(fn `UserConstructionScript`
  (`parent.UserConstructionScript`))