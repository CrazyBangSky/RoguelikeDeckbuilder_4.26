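; Component that supplies its owner's cards from a data-table attack pattern, loaded at BeginPlay along with an attack-pattern status on the owner.
; GetNextCard advances through the pattern, loops back to RepeatFrom, and makes a weighted random pick among each step's options.
; A pick that hits its consecutive-repeat limit gives way to the next option.
; Card actors are spawned lazily, cached by table and row, and destroyed with the owner.
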(event `self.ReceiveBeginPlay`
  (bind (_attackpatterndata_datatable _attackpatterndata_rowname) (break `DataTableRowHandle` (`self.AttackPatternData`)))
  (bind _returnvalue (`|GetDataTableRow` _attackpatterndata_datatable _attackpatterndata_rowname)
    (:`then`
      (bind (_cardpattern _repeatfrom) (break `/Game/RLDB/Blueprints/Structs/FCardPattern` _returnvalue))
      (set `self.AttackPattern` _cardpattern)
      (set `self.RepeatFrom` _repeatfrom)
      (add `Actor.OnDestroyed` (`self.GetOwner`) (delegate `CleanUpOnOwnerDeath`))
      (message `/Game/RLDB/Blueprints/Interfaces/BPI_CardTarget.AddToStatus` (`self.GetOwner`) "/Game/RLDB/Blueprints/Statuses/BP_Status_AttackPattern.BP_Status_AttackPattern_C" 1 false))))

(event `CleanUpOnOwnerDeath`
  (params (DestroyedActor :type "Actor Object Reference"))
  (bind _values (`BlueprintMapLibrary.Map_Values` (`self.Cards`)))
  (for _array_element _values
    (`Actor.K2_DestroyActor` _array_element)))

(fn `ChooseRandomCardOption`
  (params (CardOptions :type "/Game/RLDB/Blueprints/Structs/FCardOptions Structure"))
  (returns (Card :type "/Game/RLDB/Blueprints/Core/BP_Card Object Reference"))
  (locals (LocalWeightSum :type "Float (double-precision)") (LocalWeightSelection :type "Float (double-precision)" :default 0.0) (LocalWeightCount :type "Float (double-precision)"))
  (for _array_element (`.CardOptions_3_3400EFBB42290F98D36D25A17BB0E481` (break `/Game/RLDB/Blueprints/Structs/FCardOptions` CardOptions))
    (set `local.LocalWeightSum` (+ (`.Weight_5_8CD533564A6F5E480DC13CBA169F57BE` (break `/Game/RLDB/Blueprints/Structs/FCardOption` _array_element)) (`local.LocalWeightSum`))))
  (set `local.LocalWeightSelection` (`KismetMathLibrary.RandomFloatInRange` 0.0 (`local.LocalWeightSum`)))
  (for (_array_element_2 _array_index) (`.CardOptions_3_3400EFBB42290F98D36D25A17BB0E481` (break `/Game/RLDB/Blueprints/Structs/FCardOptions` (`local.CardOptions`)))
    (set `local.LocalWeightCount` (+ (`local.LocalWeightCount`) (`.Weight_5_8CD533564A6F5E480DC13CBA169F57BE` (break `/Game/RLDB/Blueprints/Structs/FCardOption` _array_element_2))))
    (if (>= (`local.LocalWeightCount`) (`local.LocalWeightSelection`))
      (bind _outputpin (`self.GetCardOrNextIfMaxRepeated` (break `/Game/RLDB/Blueprints/Structs/FCardOption` _array_element_2) (`.MaxRepeat_8_92E2910B41F57AAD47441191735E9998` (break `/Game/RLDB/Blueprints/Structs/FCardOption` _array_element_2)) _array_index (`local.CardOptions`)))
      (bind _output_get (set `self.PreviousPlayedCard` _outputpin))
      (return _output_get)))
  (return null))

(fn `GetCardLazy`
  (params (CardData :type "DataTableRowHandle Structure"))
  (returns (Card :type "/Game/RLDB/Blueprints/Core/BP_Card Object Reference"))
  (bind (_carddata_datatable _carddata_rowname) (break `DataTableRowHandle` (`local.CardData`)))
  (bind _returnvalue (`KismetStringLibrary.Concat_StrStr` (`KismetSystemLibrary.GetObjectName` _carddata_datatable) "," (`KismetStringLibrary.Conv_NameToString` _carddata_rowname)))
  (bind (_value _returnvalue_2) (`BlueprintMapLibrary.Map_Find` (`self.Cards`) _returnvalue))
  (if _returnvalue_2
    (`/Game/RLDB/Blueprints/Core/BP_Card.ResetInHandModifications` _value)
    (return _value)
    (else
      (bind _returnvalue_3 (`|SpawnActorFromClass` "/Game/RLDB/Blueprints/Core/BP_Card.BP_Card_C" (`KismetMathLibrary.MakeTransform` (0.0 0.0 0.0)) "AlwaysSpawn" "OverrideRootScale" (`self.GetOwner`) (`/Game/RLDB/Blueprints/Libraries/BPFL_Card.MakeCardStructFromCardData` (`local.CardData`)) null))
      (`BlueprintMapLibrary.Map_Add` (`self.Cards`) _returnvalue _returnvalue_3)
      (return _returnvalue_3))))

(fn `GetCardOrNextIfMaxRepeated`
  (params (CardData :type "DataTableRowHandle Structure") (MaxRepeat :type Integer) (CardOptionIndex :type Integer) (CardOptions :type "/Game/RLDB/Blueprints/Structs/FCardOptions Structure (by ref)"))
  (returns (OutputPin :type "/Game/RLDB/Blueprints/Core/BP_Card Object Reference"))
  (bind _output_card (break `/Game/RLDB/Blueprints/Structs/FCardOption` (`|GetArrayItem` (`.CardOptions_3_3400EFBB42290F98D36D25A17BB0E481` (break `/Game/RLDB/Blueprints/Structs/FCardOptions` (`local.CardOptions`))) (mod (+ (`local.CardOptionIndex`) 1) (`KismetArrayLibrary.Array_Length` (`.CardOptions_3_3400EFBB42290F98D36D25A17BB0E481` (break `/Game/RLDB/Blueprints/Structs/FCardOptions` (`local.CardOptions`))))))))
  (bind _card (`self.GetCardLazy` CardData))
  (if (!= (`self.PreviousPlayedCard`) _card)
    (set `self.CurrentRepetitions` 1)
    (elif (or (< (`self.CurrentRepetitions`) (`local.MaxRepeat`)) (== (`KismetArrayLibrary.Array_Length` (`self.AttackPattern`)) 0))
      (`/Engine/EditorBlueprintResources/StandardMacros.IncrementInt` (`self.CurrentRepetitions`)
        (:`  `
          _))
      (else
        (bind _card_2 (`self.GetCardLazy` _output_card))
        (set `self.CurrentRepetitions` 1)
        (return _card_2))))
  (return _card))

(fn `GetNextCard`
  (returns (Card :type "/Game/RLDB/Blueprints/Core/BP_Card Object Reference"))
  (bind _patternindex (`self.PatternIndex`))
  (`/Engine/EditorBlueprintResources/StandardMacros.IncrementInt` _patternindex
    (:`  `
      (if (not (<= _patternindex (`KismetArrayLibrary.Array_LastIndex` (`self.AttackPattern`))))
        (set `self.PatternIndex` (`self.RepeatFrom`)))
      (bind _card (`self.ChooseRandomCardOption` (`|GetArrayItem` (`self.AttackPattern`) (`self.PatternIndex`))))
      (return _card))))