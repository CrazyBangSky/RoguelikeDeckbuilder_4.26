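; Pile component for the player's hand in a card game, handling draws, discards, exhausts and resetting in-hand card modifications.
; It reacts to tagged events from a global dispatcher hub by moving cards to sibling pile components and queuing action events.
; Drawing respects a size cap in AttemptDraw, takes a specified, random or top card, and shuffles discard into draw when that pile is empty.
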(event `self.ReceiveBeginPlay`
  (`/Game/RLDB/Blueprints/Libraries/BPFL_Singletons.BindMultipleEventsToGlobalDispatcherHub` self (struct :`GameplayTags` (struct :`(TagName` "Event.Card.Discard") :`(TagName` "Event.Card.Exhaust") :`(TagName` "Event.PrePlayCard") :`(TagName` "Event.ModifyCardInHand")))))

(event `/Game/RLDB/Blueprints/Interfaces/BPI_EventHolder.RunEvent`
  (params (EventTag :type "GameplayTag Structure") (CallingObject :type "Object Object Reference (by ref)") (bGlobal :type Boolean))
  (bind _asbp_card (cast `/Game/RLDB/Blueprints/Core/BP_Card` CallingObject)
    (:`then`
      (set `self.CurrentEventCard` _asbp_card))
    (:`CastFailed`
      _))
  (`|SwitchGameplayTag` EventTag
    (:`Event.Card.Discard`
      (`self.ResolveDiscard` (`self.CurrentEventCard`)))
    (:`Event.Card.Exhaust`
      (`self.ResolveExhaust` (`self.CurrentEventCard`)))
    (:`Event.PrePlayCard`
      (message `/Game/RLDB/Blueprints/Interfaces/BPI_Pile.RemoveCardFromPile` (`Actor.GetComponentByClass` (`self.GetOwner`) "BP_PileComponent_Hand_C") (`self.CurrentEventCard`) (struct)))
    (:`Event.ModifyCardInHand`
      (`/Game/RLDB/Blueprints/Core/BP_Card.ResetInHandModifications` (`self.CurrentEventCard`)))))

(event `DiscardHand`
  (bind (_arrayindex _arrayelement) (`/Engine/EditorBlueprintResources/StandardMacros.ReverseForEachLoop` (`self.Cards`))
    (:`LoopBody`
      (`/Game/RLDB/Blueprints/Libraries/BPFL_Singletons.CallEventInGlobalDispatcherHub` (struct :`TagName` "Event.Card.Discard") _arrayelement))))

(event `AttemptDraw`
  (if (> (`self.MaxPileSize`) (`KismetArrayLibrary.Array_Length` (`self.Cards`)))
    (`self.DrawCard` null "/Game/RLDB/Blueprints/Piles/BP_PileComponent_Draw.BP_PileComponent_Draw_C")))

(fn `AddExistingCard`
  (params (Card :type "/Game/RLDB/Blueprints/Core/BP_Card Object Reference (by ref)") (TransferTag :type "GameplayTag Structure"))
  (returns (bSuccess :type Boolean))
  (bind _bsuccess (`parent.AddExistingCard` Card TransferTag))
  (if _bsuccess
    (`/Game/RLDB/Blueprints/Libraries/BPFL_Singletons.QueueEventInGlobalDispatcherHub` TransferTag Card null 0.1)
    (return true)
    (else
      (return false))))

(fn `DrawCard`
  (params (SpecifiedCard :type "/Game/RLDB/Blueprints/Core/BP_Card Object Reference") (SourcePile :type "/Game/RLDB/Blueprints/Piles/BP_PileComponent Class Reference"))
  (returns (bSuccess :type Boolean))
  (bind _drawncard (`self.DrawnCard`))
  (bind _cards (`/Game/RLDB/Blueprints/Piles/BP_PileComponent.Cards` (`Actor.GetComponentByClass` (`self.GetOwner`) (`local.SourcePile`))))
  (if (> (`KismetArrayLibrary.Array_Length` (`/Game/RLDB/Blueprints/Piles/BP_PileComponent.Cards` (`Actor.GetComponentByClass` (`self.GetOwner`) (`local.SourcePile`)))) 0)
    _
    (elif (== (`local.SourcePile`) "/Game/RLDB/Blueprints/Piles/BP_PileComponent_Draw.BP_PileComponent_Draw_C")
      (`/Game/RLDB/Blueprints/Piles/BP_PileComponent_Draw.ShuffleDiscardIntoDraw` (`Actor.GetComponentByClass` (`self.GetOwner`) "/Game/RLDB/Blueprints/Piles/BP_PileComponent_Draw.BP_PileComponent_Draw_C"))
      (if (> (`KismetArrayLibrary.Array_Length` (`/Game/RLDB/Blueprints/Piles/BP_PileComponent.Cards` (`Actor.GetComponentByClass` (`self.GetOwner`) (`local.SourcePile`)))) 0)
        _
        (else
          (return false)))
      (else
        (return false))))
  (`local.SpecifiedCard`
    (:`then`
      (if (> (`KismetArrayLibrary.Array_Find` _cards (`local.SpecifiedCard`)) -1)
        (set `self.DrawnCard` (`local.SpecifiedCard`))
        (else
          (set `self.DrawnCard` (select `bool` (`self.bRandomDrawOrder`) :`false` (`|GetArrayItem` _cards) :`true` (`KismetArrayLibrary.Array_Random` _cards)) :!label _label))))
    (:`else`
      (goto _label)))
  (`self.TransferCardToPile` (`Actor.GetComponentByClass` (`self.GetOwner`) (`local.SourcePile`)) (`self.DrawnCard`) self (struct :`TagName` "Event.Action.Draw"))
  (set `/Game/RLDB/Blueprints/Core/BP_Card.CardDataPile` (`/Game/RLDB/Blueprints/Core/BP_Card.CardDataHand` _drawncard) _drawncard)
  (`/Game/RLDB/Blueprints/Libraries/BPFL_Singletons.CallEventInGlobalDispatcherHub` (struct :`TagName` "Event.Card.Draw") (`self.DrawnCard`))
  (return true))

(fn `GetPriority`
  (returns (Priority :type "Float (double-precision)"))
  (return 100.0))

(fn `RemoveAllCardsOwnedByActor`
  (params (Actor :type "Actor Object Reference"))
  (locals (LocalCard :type "/Game/RLDB/Blueprints/Core/BP_Card Object Reference"))
  (bind _cardplayer (`/Game/RLDB/Blueprints/Libraries/BPFL_Singletons.GetCardPlayer`))
  (bind (_arrayindex _arrayelement) (`/Engine/EditorBlueprintResources/StandardMacros.ReverseForEachLoop` (`self.Cards`))
    (:`LoopBody`
      (if (== (`Actor.GetOwner` _arrayelement) Actor)
        (bind _output_get (set `local.LocalCard` _arrayelement))
        (`self.TransferCardToPile` _output_get (`/Game/RLDB/Blueprints/Core/BP_CardPlayer.BP_PileComponent_Exhaust` _cardplayer))
        (`/Game/RLDB/Blueprints/Libraries/BPFL_Singletons.QueueEventInGlobalDispatcherHub` (struct :`TagName` "Event.Action.Exhaust") (`local.LocalCard`))))
    (:`Completed`
      (return))))

(fn `ResolveDiscard`
  (params (CardToDiscard :type "/Game/RLDB/Blueprints/Core/BP_Card Object Reference"))
  (bind _returnvalue (`Actor.GetComponentByClass` (`self.GetOwner`) "/Game/RLDB/Blueprints/Piles/BP_PileComponent_Discard.BP_PileComponent_Discard_C"))
  (if (not (`KismetArrayLibrary.Array_Contains` (`/Game/RLDB/Blueprints/Piles/BP_PileComponent.Cards` _returnvalue) (`local.CardToDiscard`)))
    (`self.TransferCardToPile` (`local.CardToDiscard`) _returnvalue)
    (`/Game/RLDB/Blueprints/Libraries/BPFL_Singletons.QueueEventInGlobalDispatcherHub` (struct :`TagName` "Event.Action.Discard") (`local.CardToDiscard`))
    (`/Game/RLDB/Blueprints/Core/BP_Card.ResetInHandModifications` (`local.CardToDiscard`))
    (return)
    (else
      (return))))

(fn `ResolveExhaust`
  (params (CardToExhaust :type "/Game/RLDB/Blueprints/Core/BP_Card Object Reference"))
  (bind _returnvalue (`Actor.GetComponentByClass` (`self.GetOwner`) "/Game/RLDB/Blueprints/Piles/BP_PileComponent_Exhaust.BP_PileComponent_Exhaust_C"))
  (if (not (`KismetArrayLibrary.Array_Contains` (`/Game/RLDB/Blueprints/Piles/BP_PileComponent.Cards` _returnvalue) (`local.CardToExhaust`)))
    (`self.TransferCardToPile` (`local.CardToExhaust`) _returnvalue)
    (`/Game/RLDB/Blueprints/Libraries/BPFL_Singletons.QueueEventInGlobalDispatcherHub` (struct :`TagName` "Event.Action.Exhaust") (`local.CardToExhaust`))
    (`/Game/RLDB/Blueprints/Core/BP_Card.ResetInHandModifications` (`local.CardToExhaust`))
    (return)
    (else
      (return))))