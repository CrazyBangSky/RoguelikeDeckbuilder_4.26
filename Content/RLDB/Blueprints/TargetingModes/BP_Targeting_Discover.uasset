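; Targeting mode for Discover-style card effects that offers the player a choice of three generated cards and returns the pick as the effect's target.
; It rolls cards through the reward manager using the effect's data table rarity weights, falling back to true random, then spawns them for a reward screen.
; The Victory tag makes the screen a skippable reward.
; Confirming destroys unchosen cards; previews and non-pile targets find nothing.
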(event `BindToCardConfirm`
  (params (CardRewardScreen :type "/Game/RLDB/Widgets/WBP_CardRewardScreen Object Reference"))
  (add `/Game/RLDB/Widgets/WBP_CardRewardScreen.OnReturnSelectedCard` CardRewardScreen (delegate `ValidateAndTransferSelectedCard`)))

(event `ValidateAndTransferSelectedCard`
  (params (bSkipped :type Boolean) (Card :type "/Game/RLDB/Blueprints/Core/BP_Card Object Reference"))
  (remove `/Game/RLDB/Widgets/WBP_CardRewardScreen.OnReturnSelectedCard` (stale `BindToCardConfirm` CardRewardScreen) (delegate `ValidateAndTransferSelectedCard`))
  (for _array_element (`self.CurrentCardOptions`)
    (if (!= _array_element Card)
      (if (`KismetSystemLibrary.IsValid` _array_element)
        (`Actor.K2_DestroyActor` _array_element))))
  (if (`KismetSystemLibrary.IsValid` Card)
    (set `/Game/RLDB/Widgets/WBP_CardHand.bSelectionMode` false (`/Game/RLDB/Widgets/WBP_Layout_RLDB.WBP_Hand` (`/Game/RLDB/Blueprints/Core/BP_CardPlayer.PlayerUI` (`/Game/RLDB/Blueprints/Libraries/BPFL_Singletons.GetCardPlayerPure`))))
    (`self.OnInputTargetsReceived` (`|MakeArray` Card :!type "Actor Object Reference"))
    (else
      (`self.OnInputTargetsReceived` (`self.EmptyArray`)))))

(fn `FindValidTargets`
  (params (SpecifiedTargets :type "Array of Actor Object Reference (by ref)") (CardEffect :type "/Game/RLDB/Blueprints/Structs/FCardEffect Structure") (Card :type "/Game/RLDB/Blueprints/Core/BP_Card Object Reference") (bPreview :type Boolean))
  (returns (bTargetsFound :type Boolean) (ValidTargets :type "Array of Actor Object Reference"))
  (locals (LocalValidCards :type "Array of /Game/RLDB/Blueprints/Core/BP_Card Object Reference") (LocalCardOptions :type "Array of /Game/RLDB/Blueprints/Structs/FCard Structure") (LocalRarityWeights :type "Map of GameplayTag Structure to Float (double-precision)"))
  (bind (_useddata_datatable _useddata_rowname) (break `DataTableRowHandle` (`/Game/RLDB/Blueprints/Libraries/BPFL_CardEffect.GetEffectUsedData` (`local.CardEffect`))))
  (bind _returnvalue (`BlueprintGameplayTagLibrary.HasTag` (`/Game/RLDB/Blueprints/Libraries/BPFL_CardEffect.GetEffectGameplayTags` (`local.CardEffect`)) (struct :`TagName` "Event.Victory") true))
  (if bPreview
    (return false)
    (else
      (castclass `/Game/RLDB/Blueprints/Piles/BP_PileComponent` (`/Game/RLDB/Blueprints/Libraries/BPFL_CardEffect.GetEffectTargetComponent` CardEffect)
        (:`then`
          (`KismetArrayLibrary.Array_Clear` (`self.CurrentCardOptions`))
          (if (`KismetSystemLibrary.IsValid` _useddata_datatable)
            (bind _returnvalue_2 (`|GetDataTableRow` _useddata_datatable _useddata_rowname)
              (:`then`
                (set `local.LocalRarityWeights` (`.RarityWeights_5_FD051BF04638468B2A81C0B1F79EA934` (break `/Game/RLDB/Blueprints/Structs/FRarityWeights` _returnvalue_2)))
                (bind _randomcards (`/Game/RLDB/Blueprints/Core/BP_RewardManagerComponent.GetRandomCardsByCustomRarityWeights` (`/Game/RLDB/Blueprints/Core/BP_CardPlayer.BP_RewardManagerComponent` (`/Game/RLDB/Blueprints/Libraries/BPFL_Singletons.GetCardPlayerPure`)) (`local.LocalRarityWeights`) 3))
                (set `local.LocalCardOptions` _randomcards))
              (:`RowNotFound`
                (bind _randomcards_2 (`/Game/RLDB/Blueprints/Core/BP_RewardManagerComponent.GetTrueRandomCards` (`/Game/RLDB/Blueprints/Core/BP_CardPlayer.BP_RewardManagerComponent` (`/Game/RLDB/Blueprints/Libraries/BPFL_Singletons.GetCardPlayerPure`)) 3 :!label _label))
                (set `local.LocalCardOptions` _randomcards_2)))
            (else
              (goto _label)))
          (for _array_element (`local.LocalCardOptions`)
            (bind _returnvalue_3 (`|SpawnActorFromClass` "/Game/RLDB/Blueprints/Core/BP_Card.BP_Card_C" (`KismetMathLibrary.MakeTransform` (0.0 0.0 0.0)) "AlwaysSpawn" "OverrideRootScale" (`Actor.GetOwner` (`local.Card`)) _array_element null))
            (`KismetArrayLibrary.Array_Add` (`self.CurrentCardOptions`) _returnvalue_3))
          (`|SpawnActorFromClass` "/Game/RLDB/Blueprints/CardActions/BP_Action_RewardScreen.BP_Action_RewardScreen_C" (`KismetMathLibrary.MakeTransform` (0.0 0.0 0.0)) "AlwaysSpawn" "OverrideRootScale" null (`self.CurrentCardOptions`) (select `bool` _returnvalue :`false` "Choose a Card" :`true` "Choose your Reward!" :!type "Text") _returnvalue -1.0 null)
          (`self.BindToCardConfirm` (`/Game/RLDB/Widgets/WBP_Layout_RLDB.WBP_CardRewardScreen` (`/Game/RLDB/Blueprints/Core/BP_CardPlayer.PlayerUI` (`/Game/RLDB/Blueprints/Libraries/BPFL_Singletons.GetCardPlayerPure`))))
          (return true))
        (:`CastFailed`
          (return false))))))