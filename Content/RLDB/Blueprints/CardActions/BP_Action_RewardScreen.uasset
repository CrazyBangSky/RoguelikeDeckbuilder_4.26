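; Card action that opens the card reward screen for the acting player during play.
; On play it passes its card options, title text and skip flag to the reward screen widget on the card player's UI.
; It binds to the screen's selected-card return event and ends the action once the player picks or skips, without using the selection itself.
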(event `self.PlayAction`
  (bind _cardplayer (`/Game/RLDB/Blueprints/Libraries/BPFL_Singletons.GetCardPlayer`))
  (bind _wbp_cardrewardscreen (`/Game/RLDB/Widgets/WBP_Layout_RLDB.WBP_CardRewardScreen` (`/Game/RLDB/Blueprints/Core/BP_CardPlayer.PlayerUI` _cardplayer)))
  (add `/Game/RLDB/Widgets/WBP_CardRewardScreen.OnReturnSelectedCard` _wbp_cardrewardscreen (delegate `ContinueActionOnCardSelect`))
  (`/Game/RLDB/Widgets/WBP_CardRewardScreen.UpdateRewardScreen` _wbp_cardrewardscreen (`self.CardOptions`) (`self.ScreenText`) (`self.bAllowSkip`)))

(event `ContinueActionOnCardSelect`
  (params (bSkipped :type Boolean) (Card :type "/Game/RLDB/Blueprints/Core/BP_Card Object Reference"))
  (`self.EndAction`))

(fn `UserConstructionScript`
  (`parent.UserConstructionScript`))