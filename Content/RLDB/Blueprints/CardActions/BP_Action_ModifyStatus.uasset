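; Queued card action that visually updates a status indicator on a puppet when a status's value changes.
; SetupAction caches the status's appearance, owner, indicator and puppet up front, since the status may be destroyed before the action plays.
; PlayAction updates the indicator widget, optionally spawns icon and text splashes offset from the puppet toward the camera, then ends the action.
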(event `self.SetupAction`
  (bind _status (`self.Status`))
  (bind _returnvalue (`ActorComponent.GetOwner` _status))
  ;[0 0 0] Store variables from status that will be used for display when playing the action. Done here instead of getting these from the Status directly during Play Action as the status might be destroyed between queueing and playing the action, which will make the reference invalid
  (bind _statusappearance (`/Game/RLDB/Blueprints/Statuses/BP_Status.MakeAppearanceStruct` _status))
  (set `self.Status Appearance` _statusappearance)
  (set `self.StatusOwner` _returnvalue)
  (set `self.StatusIndicator` (`/Game/RLDB/Blueprints/Statuses/BP_Status.StatusIndicator` _status))
  (bind _puppet (message `/Game/RLDB/Blueprints/Interfaces/BPI_CardTarget.GetPuppet` _returnvalue))
  (set `self.Puppet` _puppet))

(event `self.PlayAction`
  (bind _puppet (`self.Puppet`))
  (bind _puppet_2 (`self.Puppet`))
  (bind ((`Icon_2_3CC270F545FEEDAA11FCB7B11FCC6857` _icon) (`Tint_11_593025904124C15E45BC999B5974F503` _tint)) (break `/Game/RLDB/Blueprints/Structs/FStatusAppearance` (`self.Status Appearance`)))
  (message `/Game/RLDB/Blueprints/Interfaces/BPI_StatusIcon.ModifyStatusWidget` (`self.StatusIndicator`) (`self.NewValue`) (`self.Text Override`) (`self.bRefreshAppearance`) (`self.Status Appearance`))
  (`|ExecutionSequence`
    (:`then_0`
      (if (`self.bShowSplashIcon`)
        (bind _relativecenter (message `/Game/RLDB/Blueprints/Interfaces/BPI_CardPuppet.GetPuppetRelativeCenter` _puppet))
        (`|SpawnActorFromClass` "/Game/RLDB/Blueprints/UI/BP_IconSplash.BP_IconSplash_C" (`KismetMathLibrary.MakeTransform` (`KismetMathLibrary.VLerp` (+ _relativecenter (`self.K2_GetActorLocation` _puppet)) (`PlayerCameraManager.GetCameraLocation` (`GameplayStatics.GetPlayerCameraManager` 0)) 0.2)) "AlwaysSpawn" "OverrideRootScale" null _icon _tint null)))
    (:`then_1`
      (if (and (`self.bShowSplashNumber`) (not (`KismetTextLibrary.TextIsEmpty` (`self.SplashText`))))
        (bind _relativecenter_2 (message `/Game/RLDB/Blueprints/Interfaces/BPI_CardPuppet.GetPuppetRelativeCenter` _puppet_2))
        (`|SpawnActorFromClass` "/Game/RLDB/Blueprints/UI/BP_TextSplash.BP_TextSplash_C" (`KismetMathLibrary.MakeTransform` (+ (`KismetMathLibrary.VLerp` (+ _relativecenter_2 (`self.K2_GetActorLocation` _puppet_2)) (`PlayerCameraManager.GetCameraLocation` (`GameplayStatics.GetPlayerCameraManager` 0)) 0.2) (0.0 0.0 70.0)) (struct :`Yaw` 90.0)) "AlwaysSpawn" "OverrideRootScale" null (`self.SplashText`) (`KismetMathLibrary.Conv_LinearColorToColor` (`.Tint_11_593025904124C15E45BC999B5974F503` (break `/Game/RLDB/Blueprints/Structs/FStatusAppearance` (`self.Status Appearance`)))) null))
      (`self.EndAction`))))

(fn `UserConstructionScript`
  (`parent.UserConstructionScript`))