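; Card action that pops floating splash text over the puppet that performs it.
; On play it spawns a BP_TextSplash actor slightly above the puppet's relative center-message point, passing along the configured text and color.
; It ends the action immediately after spawning, without waiting for the splash to finish.
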(event `self.PlayAction`
  (bind _puppet (`self.Puppet`))
  (bind _relativecenter (message `/Game/RLDB/Blueprints/Interfaces/BPI_CardPuppet.GetPuppetRelativeCenter` _puppet))
  (`|SpawnActorFromClass` "/Game/RLDB/Blueprints/UI/BP_TextSplash.BP_TextSplash_C" (`KismetMathLibrary.MakeTransform` (+ (+ _relativecenter (`self.K2_GetActorLocation` _puppet)) (0.0 0.0 70.0))) "Undefined" "OverrideRootScale" null (`self.DisplayText`) (`KismetMathLibrary.Conv_LinearColorToColor` (`self.Color`)) null)
  (`self.EndAction`))

(fn `UserConstructionScript`
  (`parent.UserConstructionScript`))