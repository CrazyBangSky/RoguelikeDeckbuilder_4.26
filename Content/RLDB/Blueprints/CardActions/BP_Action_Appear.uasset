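; Card action Blueprint that makes its puppet appear or disappear.
; PlayAction checks the Disappear flag and sends the matching appear or disappear message with FadeSpeed to the Puppet, which handles the animation and display itself.
; It calls EndAction immediately after sending the message, without waiting for the fade to finish.
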(event `self.PlayAction`
  ;[0 0 0] Calls on the puppet to appear or disappear depending on the input. The puppet handles how to animate/display these events
  (if (`self.bDisappear`)
    (message `/Game/RLDB/Blueprints/Interfaces/BPI_CardPuppet.DisappearPuppet` (`self.Puppet`) (`self.FadeSpeed`))
    (else
      (message `/Game/RLDB/Blueprints/Interfaces/BPI_CardPuppet.AppearPuppet` (`self.Puppet`) (`self.FadeSpeed`))))
  (`self.EndAction`))

(fn `UserConstructionScript`
  (`parent.UserConstructionScript`))