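; BP_Action_LoadMap is a card action that fades out the screen and then loads another map.
; On PlayAction it creates a WBP_ScreenFade widget, adds it to the viewport and plays its Occlude animation.
; It waits just past that animation's end time, then opens the level named by its Level variable.
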(event `self.PlayAction`
  (bind _returnvalue (`|CreateWidget` "/Game/RLDB/Widgets/WBP_ScreenFade.WBP_ScreenFade_C"))
  (`UserWidget.AddToViewport` _returnvalue 0)
  (bind _occlude (`/Game/RLDB/Widgets/WBP_ScreenFade.Occlude` _returnvalue))
  (`UserWidget.PlayAnimation` _returnvalue _occlude 0.0 1 "Forward" 1.0 false)
  (`KismetSystemLibrary.Delay` (+ (`WidgetAnimation.GetEndTime` _occlude) 0.01))
  (`GameplayStatics.OpenLevel` (`KismetStringLibrary.Conv_StringToName` (`self.Level`))))

(fn `UserConstructionScript`
  (`parent.UserConstructionScript`))