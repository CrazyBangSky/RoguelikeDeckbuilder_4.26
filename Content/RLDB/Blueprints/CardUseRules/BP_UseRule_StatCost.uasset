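; Card use rule that makes playing a card cost the card player's stats, using the parent card's use costs keyed by status component class.
; The check fails if the player lacks any required status component or its value is too low, returning a "Not Enough" message in the latter case.
; Resolving subtracts each cost with a splash display, then queues a ResourceChange event in the global dispatcher hub.
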(fn `CheckIfUseAllowed`
  (returns (bAllowed :type Boolean) (FailMessage :type String))
  (bind _cardplayer (`/Game/RLDB/Blueprints/Libraries/BPFL_Singletons.GetCardPlayer`))
  (bind _keys (`BlueprintMapLibrary.Map_Keys` (`/Game/RLDB/Blueprints/Core/BP_Card.GetCardUseCosts` (`self.ParentCard`) "NewEnumerator0")))
  (for _array_element _keys
    (bind _returnvalue (`Actor.GetComponentByClass` _cardplayer _array_element))
    (if (`KismetSystemLibrary.IsValid` _returnvalue)
      (if (not (>= (`/Game/RLDB/Blueprints/Statuses/BP_Status.StatusValue` _returnvalue) (`BlueprintMapLibrary.Map_Find` (`/Game/RLDB/Blueprints/Core/BP_Card.GetCardUseCosts` (`self.ParentCard`) "NewEnumerator0") _array_element)))
        (return false (`KismetStringLibrary.Concat_StrStr` "Not Enough " (`KismetTextLibrary.Conv_TextToString` (`/Game/RLDB/Blueprints/Statuses/BP_Status.FriendlyName` _returnvalue)))))
      (else
        (return false ""))))
  (return true ""))

(fn `ResolveUseConsequence`
  (returns (bSuccess :type Boolean))
  (bind _usecosts (`/Game/RLDB/Blueprints/Core/BP_Card.GetCardUseCosts` (`self.ParentCard`) "NewEnumerator0"))
  (bind _cardplayer (`/Game/RLDB/Blueprints/Libraries/BPFL_Singletons.GetCardPlayer`))
  (bind _keys (`BlueprintMapLibrary.Map_Keys` _usecosts))
  (for _array_element _keys
    (message `/Game/RLDB/Blueprints/Interfaces/BPI_CardTarget.SubtractFromStatus` _cardplayer _array_element (`BlueprintMapLibrary.Map_Find` _usecosts _array_element) true))
  (bind _bsuccess (`/Game/RLDB/Blueprints/Libraries/BPFL_Singletons.QueueEventInGlobalDispatcherHub` (struct :`TagName` "Event.Action.ResourceChange") self))
  (return _bsuccess))