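; BP_CardEffect appears to be the base Blueprint for card effects, providing shared targeting setup and resolution hooks.
; On BeginPlay it falls back to DefaultTargetingClass when TargetingClass is invalid.
; InitializeCardEffect is an empty stub, and ResolveCardEffect takes a target actor and simply returns true.
; Interrupt and CancelInterruption both set the Interrupt flag to true, so cancelling does not clear it.
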(event `self.ReceiveBeginPlay`
  (if (not (`KismetSystemLibrary.IsValidClass` (`self.TargetingClass`)))
    (set `self.TargetingClass` (`self.DefaultTargetingClass`))))

(event `/Game/RLDB/Blueprints/Interfaces/BPI_Interrupt.Interrupt`
  (set `self.bInterrupt` true))

(event `/Game/RLDB/Blueprints/Interfaces/BPI_Interrupt.CancelInterruption`
  (set `self.bInterrupt` true))

(fn `InitializeCardEffect`
  (return))

(fn `ResolveCardEffect`
  (params (TargetActor :type "Actor Object Reference"))
  (returns (bSuccess :type Boolean))
  (return true))