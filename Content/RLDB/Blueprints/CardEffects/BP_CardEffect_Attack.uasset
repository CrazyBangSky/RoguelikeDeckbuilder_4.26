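; Card effect that attacks a target actor, subtracting the effect value from its health status with a splash number.
; Fires pre-attack and post-attack events on the card owner's dispatcher hub and an incoming-attack event on the target's hub, passing itself as the calling object.
; The pre-attack hook lets other Blueprints modify the attack before damage lands.
; A screen shake action spawns, scaled by damage size.
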(fn `ResolveCardEffect`
  (params (TargetActor :type "Actor Object Reference"))
  (returns (bSuccess :type Boolean))
  (locals (LocalArmor :type Integer))
  (bind _returnvalue (`Actor.GetComponentByClass` (`self.AttackTarget`) "/Game/RLDB/Blueprints/Statuses/BP_Status_Health.BP_Status_Health_C"))
  (set `self.AttackTarget` TargetActor)
  (bind _parentcard (`self.ParentCard`)
    (:`then`
      (bind _returnvalue_2 (`Actor.GetComponentByClass` (`Actor.GetOwner` _parentcard) "/Game/RLDB/Blueprints/Core/BP_DispatcherHubComponent.BP_DispatcherHubComponent_C"))
      (`/Engine/EditorBlueprintResources/StandardMacros.IsValid` _returnvalue_2
        (:`Is Valid`
          (`/Game/RLDB/Blueprints/Core/BP_DispatcherHubComponent.CallBoundEvents` _returnvalue_2 (struct :`TagName` "Event.PreAttack") self null true) ; Calls event to any blueprint that might want to modify the attack before it happens,\npassing the card effects as the calling object
        )
        (:`Is Not Valid`
          _)))
    (:`else`
      _))
  (`|SpawnActorFromClass` "/Game/RLDB/Blueprints/CardActions/BP_Action_ScreenShake.BP_Action_ScreenShake_C" (`KismetMathLibrary.MakeTransform` (0.0 0.0 0.0)) "Undefined" "OverrideRootScale" null (* (`KismetMathLibrary.Conv_IntToDouble` (`KismetMathLibrary.Abs_Int` (`self.EffectValue`))) (`self.DamageScaleFactor`)) "/Game/RLDB/Blueprints/UI/BP_ScreenShake.BP_ScreenShake_C" -1.0 null)
  (`/Game/RLDB/Blueprints/Core/BP_DispatcherHubComponent.CallBoundEvents` (`Actor.GetComponentByClass` (`self.AttackTarget`) "/Game/RLDB/Blueprints/Core/BP_DispatcherHubComponent.BP_DispatcherHubComponent_C") (struct :`TagName` "Event.IncomingAttack") self null true)
  (`/Engine/EditorBlueprintResources/StandardMacros.IsValid` _returnvalue
    (:`Is Valid`
      (`/Game/RLDB/Blueprints/Statuses/BP_Status.SubtractStatusValue` _returnvalue (`self.EffectValue`) true false))
    (:`Is Not Valid`
      _))
  (bind _parentcard_2 (`self.ParentCard`)
    (:`then`
      (bind _returnvalue_3 (`Actor.GetOwner` _parentcard_2))
      (`/Engine/EditorBlueprintResources/StandardMacros.IsValid` _returnvalue_3
        (:`Is Valid`
          (bind _returnvalue_4 (`Actor.GetComponentByClass` _returnvalue_3 "/Game/RLDB/Blueprints/Core/BP_DispatcherHubComponent.BP_DispatcherHubComponent_C"))
          (`/Engine/EditorBlueprintResources/StandardMacros.IsValid` _returnvalue_4
            (:`Is Valid`
              (`/Game/RLDB/Blueprints/Core/BP_DispatcherHubComponent.CallBoundEvents` _returnvalue_4 (struct :`TagName` "Event.PostAttack") self null true))
            (:`Is Not Valid`
              _)))
        (:`Is Not Valid`
          _)))
    (:`else`
      _))
  (return true))