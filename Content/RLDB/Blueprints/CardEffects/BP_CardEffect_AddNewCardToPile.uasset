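; Card effect that generates a card into one of the card player's piles, chosen by TargetComponent and defaulting to the hand.
; Uses the target actor if it is a card, otherwise spawns one from the UsedData data table reference.
; Fires the global Generate event and messages the pile once per EffectValue, reusing that same card instance.
; Returns false when EffectValue is not positive or no card source exists.
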(fn `ResolveCardEffect`
  (params (TargetActor :type "Actor Object Reference"))
  (returns (bSuccess :type Boolean))
  (locals (LocalTargetPileClass :type "/Game/RLDB/Blueprints/Piles/BP_PileComponent Object Reference") (LocalCard :type "/Game/RLDB/Blueprints/Core/BP_Card Object Reference"))
  (bind _useddata_datatable (break `DataTableRowHandle` (`self.UsedData`)))
  ;[0 0 0] Takes either a card reference, or if none is available a reference to a card in a data table, and attempts to add to the specified pile (set in TargetComponent)
  (bind _asbp_card (cast `/Game/RLDB/Blueprints/Core/BP_Card` TargetActor)
    (:`then`
      (set `local.LocalCard` _asbp_card))
    (:`CastFailed`
      (if (`KismetSystemLibrary.IsValid` _useddata_datatable)
        (bind _returnvalue (`|SpawnActorFromClass` "/Game/RLDB/Blueprints/Core/BP_Card.BP_Card_C" (`KismetMathLibrary.MakeTransform` (0.0 0.0 0.0)) "AlwaysSpawn" "OverrideRootScale" (`Actor.GetOwner` (`self.ParentCard`)) (`/Game/RLDB/Blueprints/Libraries/BPFL_Card.MakeCardStructFromCardData` (`self.UsedData`)) null))
        (set `local.LocalCard` _returnvalue)
        (else
          (return false)))))
  (if (> (`self.EffectValue`) 0)
    (bind _asbp_pile_component (castclass `/Game/RLDB/Blueprints/Piles/BP_PileComponent` (`self.TargetComponent`)) ; If no pile is specified, adds to hand
      (:`then`
        (set `local.LocalTargetPileClass` _asbp_pile_component))
      (:`CastFailed`
        (set `local.LocalTargetPileClass` "/Game/RLDB/Blueprints/Piles/BP_PileComponent_Hand.BP_PileComponent_Hand_C")))
    (for _ (range 1 (+ (`self.EffectValue`) 1))
      (`/Game/RLDB/Blueprints/Libraries/BPFL_Singletons.CallEventInGlobalDispatcherHub` (struct :`TagName` "Event.Card.Generate") (`local.LocalCard`))
      (message `/Game/RLDB/Blueprints/Interfaces/BPI_Pile.AddExistingCard` (`Actor.GetComponentByClass` (`/Game/RLDB/Blueprints/Libraries/BPFL_Singletons.GetCardPlayerPure`) (`local.LocalTargetPileClass`)) (`local.LocalCard`) (struct :`TagName` "Event.Action.GenerateCard")))
    (return true)
    (else
      (return false))))