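; Card effect that changes an attack card's damage both in hand and in pile, so the change is not reset on discard.
; ResolveCardEffect casts the target to BP_Card and applies EffectValue through ModifyCardAttackDamage twice, once per modification type.
; It then raises the ModifyCardInHand event through the global dispatcher hub and returns true, or returns false for non-card targets.
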(fn `ResolveCardEffect`
  (params (TargetActor :type "Actor Object Reference"))
  (returns (bSuccess :type Boolean))
  (locals (LocalEffects :type "Array of /Game/RLDB/Blueprints/Structs/FCardEffect Structure") (LocalCard :type "/Game/RLDB/Blueprints/Core/BP_Card Object Reference") (bLocalCardModified :type Boolean))
  ;[0 0 0] Changes the damage of an attack card, both in hand and in pile (is not reset when discarded)
  (bind _asbp_card (cast `/Game/RLDB/Blueprints/Core/BP_Card` TargetActor)
    (:`then`
      (bind _output_get (set `local.LocalCard` _asbp_card))
      (`/Game/RLDB/Blueprints/Core/BP_Card.ModifyCardAttackDamage` _output_get (`self.EffectValue`) "NewEnumerator0")
      (`/Game/RLDB/Blueprints/Core/BP_Card.ModifyCardAttackDamage` (`local.LocalCard`) (`self.EffectValue`) "NewEnumerator3")
      (`/Game/RLDB/Blueprints/Libraries/BPFL_Singletons.CallEventInGlobalDispatcherHub` (struct :`TagName` "Event.ModifyCardInHand") (`local.LocalCard`))
      (return true))
    (:`CastFailed`
      (return false))))